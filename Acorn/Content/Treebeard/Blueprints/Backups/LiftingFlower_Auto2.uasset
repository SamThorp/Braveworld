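; Flower actor that reacts to hits from a SeedWater actor by opening petals and, unless Unmoving, lifting its Centre toward EndVector.
; A sphere hit either opens and closes the petals around a StayUpTime delay, or starts a guarded Timeline that lerps Centre, then reverses after that delay.
; Petal events toggle collision and play an animation, though closing reuses the open animation and opening leaves Petal3's collision off.
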(event `self.ReceiveBeginPlay`
  (`PrimitiveComponent.SetCollisionEnabled` (`self.Petal1`) "NoCollision")
  (`PrimitiveComponent.SetCollisionEnabled` (`self.Petal2`) "NoCollision")
  (`PrimitiveComponent.SetCollisionEnabled` (`self.Petal3`) "NoCollision")
  (set `self.StartVector` (0.0 0.0 0.0)))

(event `OpenPetal`
  (`SkeletalMeshComponent.PlayAnimation` (`self.SkeletalMesh`) "/Game/_ProjectTreebeard/ElenaModels/Lily/FlowerAnimOpen_Anim.FlowerAnimOpen_Anim" false)
  (`PrimitiveComponent.SetCollisionEnabled` (`self.Petal1`) "QueryAndPhysics")
  (`PrimitiveComponent.SetCollisionEnabled` (`self.Petal2`) "QueryAndPhysics"))

(event `ClosePetal`
  (`SkeletalMeshComponent.PlayAnimation` (`self.SkeletalMesh`) "/Game/_ProjectTreebeard/ElenaModels/Lily/FlowerAnimOpen_Anim.FlowerAnimOpen_Anim" false)
  (`PrimitiveComponent.SetCollisionEnabled` (`self.Petal1`) "NoCollision")
  (`PrimitiveComponent.SetCollisionEnabled` (`self.Petal2`) "NoCollision")
  (`PrimitiveComponent.SetCollisionEnabled` (`self.Petal3`) "NoCollision"))

(event `self.Sphere.OnComponentHit`
  (params (HitComponent :type "PrimitiveComponent Object Reference") (OtherActor :type "Actor Object Reference") (OtherComp :type "PrimitiveComponent Object Reference") (NormalImpulse :type "Vector Structure") (Hit :type "HitResult Structure (by ref)"))
  (cast `/Game/Treebeard/Blueprints/Player/Seeds/SeedWater` OtherActor)
  (`KismetSystemLibrary.PrintString` "Hello")
  (if (`self.Unmoving`)
    (`self.OpenPetal`)
    (`KismetSystemLibrary.Delay` (`self.StayUpTime`))
    (`self.ClosePetal`)
    (elif (not (`self.Moving`))
      (`|ExecutionSequence`
        (:`then_0`
          (goto _label :!via `Reset`))
        (:`then_1`
          (`/Engine/EditorBlueprintResources/StandardMacros.DoOnce` false :!label _label
            (:`Completed`
              (set `self.Moving` true)
              (bind (_direction _swivel) (`Timeline|Timeline_0` :!label _label_2)
                (:`Update`
                  (`SceneComponent.K2_SetRelativeLocation` (`self.Centre`) (`KismetMathLibrary.VLerp` (`self.StartVector`) (`self.EndVector`) (/ _swivel (`self.Speed`))) false false))
                (:`Finished`
                  (`|ExecutionSequence`
                    (:`then_0`
                      (if (== _swivel 100.0)
                        (`self.OpenPetal`)
                        (else
                          (`self.ClosePetal`))))
                    (:`then_1`
                      (if (`self.Moving`)
                        (`KismetSystemLibrary.Delay` (`self.StayUpTime`))
                        (set `self.Moving` false)
                        (goto _label_2 :!via `Reverse`)
                        (else
                          (goto _label_2 :!via `SetNewTime`))))))))))))))

(fn `UserConstructionScript`)