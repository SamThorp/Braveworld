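; A giant flower actor that blooms once SeedWater hits on its six bulbs bring Health to zero.
; Each hit hides and disables that bulb, spawns a water burst effect and decrements Health.
; An Unmoving flower opens its petals in place, toggling visibility and some collision, then closes after StayUpTime.
; Otherwise a timeline moves Centre toward EndVector, opens the petals, waits, then reverses and closes them.
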(event `self.ReceiveBeginPlay`
  (`PrimitiveComponent.SetCollisionEnabled` (`self.Petal1`) "NoCollision")
  (`PrimitiveComponent.SetCollisionEnabled` (`self.Petal2`) "NoCollision")
  (`PrimitiveComponent.SetCollisionEnabled` (`self.Petal3`) "NoCollision")
  (set `self.StartVector` (0.0 0.0 0.0)))

(event `self.Bulb1.OnComponentHit`
  (params (HitComponent :type "PrimitiveComponent Object Reference") (OtherActor :type "Actor Object Reference") (OtherComp :type "PrimitiveComponent Object Reference") (NormalImpulse :type "Vector Structure") (Hit :type "HitResult Structure (by ref)"))
  (`self.SeedHit` OtherActor (`self.Bulb1`)))

(event `OpenPetal`
  (bind _bulb (`self.Bulb`))
  (bind _petal1 (`self.Petal1`))
  (`SceneComponent.SetVisibility` _petal1 true false)
  (`SceneComponent.SetVisibility` (`self.Petal2`) true false)
  (`SceneComponent.SetVisibility` (`self.Petal3`) true false)
  (`SceneComponent.SetVisibility` (`self.Petal4`) true false)
  (`SceneComponent.SetVisibility` (`self.Petal5`) true false)
  (`SceneComponent.SetVisibility` (`self.Petal6`) true false)
  (`SceneComponent.SetVisibility` (`self.Petal7`) true false)
  (`SceneComponent.SetVisibility` (`self.Petal8`) true false)
  (`SceneComponent.SetVisibility` (`self.Petal9`) true false)
  (`PrimitiveComponent.SetCollisionEnabled` _petal1 "QueryAndPhysics")
  (`PrimitiveComponent.SetCollisionEnabled` (`self.Petal2`) "QueryAndPhysics")
  (`SceneComponent.SetVisibility` _bulb false false)
  (`PrimitiveComponent.SetCollisionEnabled` _bulb "NoCollision"))

(event `ClosePetal`
  (bind _bulb (`self.Bulb`))
  (bind _petal1 (`self.Petal1`))
  (`SceneComponent.SetVisibility` _petal1 false false)
  (`SceneComponent.SetVisibility` (`self.Petal2`) false false)
  (`SceneComponent.SetVisibility` (`self.Petal3`) false false)
  (`SceneComponent.SetVisibility` (`self.Petal9`) false false)
  (`SceneComponent.SetVisibility` (`self.Petal8`) false false)
  (`SceneComponent.SetVisibility` (`self.Petal7`) false false)
  (`SceneComponent.SetVisibility` (`self.Petal5`) false false)
  (`SceneComponent.SetVisibility` (`self.Petal4`) false false)
  (`PrimitiveComponent.SetCollisionEnabled` _petal1 "NoCollision")
  (`PrimitiveComponent.SetCollisionEnabled` (`self.Petal2`) "NoCollision")
  (`PrimitiveComponent.SetCollisionEnabled` (`self.Petal3`) "NoCollision")
  (`SceneComponent.SetVisibility` _bulb true false)
  (`PrimitiveComponent.SetCollisionEnabled` _bulb "QueryAndPhysics"))

(event `self.Bulb2.OnComponentHit`
  (params (HitComponent :type "PrimitiveComponent Object Reference") (OtherActor :type "Actor Object Reference") (OtherComp :type "PrimitiveComponent Object Reference") (NormalImpulse :type "Vector Structure") (Hit :type "HitResult Structure (by ref)"))
  (`self.SeedHit` OtherActor (`self.Bulb2`)))

(event `SeedHit`
  (params (Seed :type "Actor Object Reference") (Bulb :type "StaticMeshComponent Object Reference"))
  (bind _health (`self.Health`))
  (cast `/Game/Treebeard/Blueprints/Player/Seeds/SeedWater` Seed)
  (`SceneComponent.SetHiddenInGame` Bulb true false)
  (`GameplayStatics.SpawnEmitterAtLocation` "/Game/InfinityBladeEffects/ForTreebeard/P_WaterBoomFlower.P_WaterBoomFlower" (`SceneComponent.K2_GetComponentLocation` Bulb) (`SceneComponent.K2_GetComponentRotation` Bulb) (4.0 4.0 4.0))
  (`PrimitiveComponent.SetCollisionEnabled` Bulb "NoCollision")
  (`/Engine/EditorBlueprintResources/StandardMacros.DecrementInt` _health
    (:`  `
      (if (== _health 0)
        (if (`self.Unmoving`)
          (`self.OpenPetal`)
          (`KismetSystemLibrary.Delay` (`self.StayUpTime`))
          (`self.ClosePetal`)
          (elif (not (`self.Moving`))
            (`|ExecutionSequence`
              (:`then_0`
                (goto _label :!via `Reset`))
              (:`then_1`
                (`/Engine/EditorBlueprintResources/StandardMacros.DoOnce` false :!label _label
                  (:`Completed`
                    (set `self.Moving` true)
                    (bind (_direction _swivel) (`Timeline|Timeline_0` :!label _label_2)
                      (:`Update`
                        (`SceneComponent.K2_SetRelativeLocation` (`self.Centre`) (`KismetMathLibrary.VLerp` (`self.StartVector`) (`self.EndVector`) (/ _swivel (`self.Speed`))) false false))
                      (:`Finished`
                        (`|ExecutionSequence`
                          (:`then_0`
                            (if (== _swivel 100.0)
                              (`self.OpenPetal`)
                              (else
                                (`self.ClosePetal`))))
                          (:`then_1`
                            (if (`self.Moving`)
                              (`KismetSystemLibrary.Delay` (`self.StayUpTime`))
                              (set `self.Moving` false)
                              (goto _label_2 :!via `Reverse`)
                              (else
                                (goto _label_2 :!via `SetNewTime`)))))))))))))))))

(event `self.Bulb3.OnComponentHit`
  (params (HitComponent :type "PrimitiveComponent Object Reference") (OtherActor :type "Actor Object Reference") (OtherComp :type "PrimitiveComponent Object Reference") (NormalImpulse :type "Vector Structure") (Hit :type "HitResult Structure (by ref)"))
  (`self.SeedHit` OtherActor (`self.Bulb3`)))

(event `self.Bulb4.OnComponentHit`
  (params (HitComponent :type "PrimitiveComponent Object Reference") (OtherActor :type "Actor Object Reference") (OtherComp :type "PrimitiveComponent Object Reference") (NormalImpulse :type "Vector Structure") (Hit :type "HitResult Structure (by ref)"))
  (`self.SeedHit` OtherActor (`self.Bulb4`)))

(event `self.Bulb5.OnComponentHit`
  (params (HitComponent :type "PrimitiveComponent Object Reference") (OtherActor :type "Actor Object Reference") (OtherComp :type "PrimitiveComponent Object Reference") (NormalImpulse :type "Vector Structure") (Hit :type "HitResult Structure (by ref)"))
  (`self.SeedHit` OtherActor (`self.Bulb5`)))

(event `self.Bulb6.OnComponentHit`
  (params (HitComponent :type "PrimitiveComponent Object Reference") (OtherActor :type "Actor Object Reference") (OtherComp :type "PrimitiveComponent Object Reference") (NormalImpulse :type "Vector Structure") (Hit :type "HitResult Structure (by ref)"))
  (`self.SeedHit` OtherActor (`self.Bulb6`)))

(fn `UserConstructionScript`)