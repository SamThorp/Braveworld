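; Gong is an actor that reacts to being hit by seeds and makes a linked game object disappear.
; Each hit from an AnySeed spawns an enlarged gong particle effect at the mesh and plays the gong sound.
; On the first such hit only, a DoOnce gate hides the referenced GameObject, disables its collision and plays a disappear sound at its location.
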(event `self.ReceiveHit`
  (params (MyComp :type "PrimitiveComponent Object Reference") (Other :type "Actor Object Reference") (OtherComp :type "PrimitiveComponent Object Reference") (bSelfMoved :type Boolean) (HitLocation :type "Vector Structure") (HitNormal :type "Vector Structure") (NormalImpulse :type "Vector Structure") (Hit :type "HitResult Structure (by ref)"))
  (bind _gameobject (`self.GameObject`))
  (bind _staticmeshcomponent (`self.StaticMeshComponent`))
  (cast `/Game/Treebeard/Blueprints/Player/Seeds/AnySeed` Other)
  (`GameplayStatics.SpawnEmitterAtLocation` "/Game/StarterContent/Particles/P_SoundGong.P_SoundGong" (`SceneComponent.K2_GetComponentLocation` _staticmeshcomponent) (`SceneComponent.K2_GetComponentRotation` _staticmeshcomponent) (1.5 1.5 1.5))
  (`GameplayStatics.PlaySoundAtLocation` "/Game/_Sounds/Royalty_Free_Audio/AudioCues/S_Gong_Cue.S_Gong_Cue" (`self.K2_GetActorLocation`) (struct) 1.0 1.0 0.0 null null null)
  (`/Engine/EditorBlueprintResources/StandardMacros.DoOnce` false
    (:`Completed`
      (`self.SetActorHiddenInGame` _gameobject true)
      (`self.SetActorEnableCollision` _gameobject false)
      (`GameplayStatics.PlaySoundAtLocation` "/Game/_Sounds/Royalty_Free_Audio/AudioCues/S_ObjectDisappear_Cue.S_ObjectDisappear_Cue" (`self.K2_GetActorLocation` (`self.GameObject`)) (struct) 1.0 1.0 0.0 null null null))))

(fn `UserConstructionScript`)