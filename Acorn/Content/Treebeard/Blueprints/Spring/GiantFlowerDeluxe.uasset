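; Giant flower that opens once its parasite Health count reaches zero, swapping collision from bulb to petals, then closes after StayUpTime.
; Unmoving flowers open in place; others slide Centre to EndVector on a timeline, open, then reverse and close.
; Opening plays animations and a vine-destroy sound at a linked GameObject.
; Deluxe flowers also darken that object's material in steps, show a reminder message, then hide it with a particle burst.
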(event `self.ReceiveBeginPlay`
  (`PrimitiveComponent.SetCollisionEnabled` (`self.Petal1`) "NoCollision")
  (`PrimitiveComponent.SetCollisionEnabled` (`self.Petal2`) "NoCollision")
  (`PrimitiveComponent.SetCollisionEnabled` (`self.Petal3`) "NoCollision")
  (set `self.StartVector` (0.0 0.0 0.0))
  (`SkeletalMeshComponent.PlayAnimation` (`self.SkeletalMesh1`) "/Game/_ProjectTreebeard/ElenaModels/Lily/FlowerAnimClose_Anim.FlowerAnimClose_Anim" false)
  (`SkeletalMeshComponent.PlayAnimation` (`self.SkeletalMesh`) "/Game/_ProjectTreebeard/ElenaModels/Lily/FlowerAnimClose_Anim.FlowerAnimClose_Anim" false))

(event `OpenPetal`
  (bind _gameobject (`self.GameObject`))
  (`PrimitiveComponent.SetCollisionEnabled` (`self.Petal1`) "QueryAndPhysics")
  (`PrimitiveComponent.SetCollisionEnabled` (`self.Petal2`) "QueryAndPhysics")
  (`PrimitiveComponent.SetCollisionEnabled` (`self.Bulb`) "NoCollision")
  (`SkeletalMeshComponent.PlayAnimation` (`self.SkeletalMesh1`) "/Game/_ProjectTreebeard/ElenaModels/Lily/FlowerAnimOpen_Anim.FlowerAnimOpen_Anim" false)
  (`SkeletalMeshComponent.PlayAnimation` (`self.SkeletalMesh`) "/Game/_ProjectTreebeard/ElenaModels/Lily/FlowerAnimOpen_Anim.FlowerAnimOpen_Anim" false)
  (`KismetSystemLibrary.Delay` 2.5)
  (`GameplayStatics.PlaySoundAtLocation` "/Game/_Sounds/Royalty_Free_Audio/AudioCues/S_IvyDestroy.S_IvyDestroy" (`self.K2_GetActorLocation` (`self.GameObject`)) (struct) 1.0 1.0 0.0 null null null)
  (if (`self.Deluxe`)
    (bind _asstatic_mesh_actor (cast `StaticMeshActor` _gameobject)
      (:`then`
        (bind _staticmeshcomponent (`StaticMeshActor.StaticMeshComponent` _asstatic_mesh_actor))
        (`PrimitiveComponent.SetMaterial` _staticmeshcomponent 0 "/Game/_StylizedContent/Stylized_Landscape/materials/plants_materials/MI_vines_InstDarkA.MI_vines_InstDarkA")
        (`KismetSystemLibrary.Delay` 0.45)
        (`PrimitiveComponent.SetMaterial` _staticmeshcomponent 0 "/Game/_StylizedContent/Stylized_Landscape/materials/plants_materials/MI_vines_InstDarkB.MI_vines_InstDarkB")
        (`KismetSystemLibrary.Delay` 0.45)
        (bind _asmain_character (cast `/Game/Treebeard/Blueprints/Player/MainCharacter` (`GameplayStatics.GetPlayerCharacter` 0)))
        (`/Game/Treebeard/Blueprints/Player/MainCharacter.CheckpointLevelName` _asmain_character (`self.Reminder`) (`self.Content`) "/Game/Font/Frostys_Winterland_Font.Frostys_Winterland_Font" 0.5)
        (`PrimitiveComponent.SetMaterial` _staticmeshcomponent 0 "/Game/_StylizedContent/Stylized_Landscape/materials/plants_materials/MI_vines_InstDarkC.MI_vines_InstDarkC")
        (`KismetSystemLibrary.Delay` 0.45))
      (:`CastFailed`
        _))
    (`self.SetActorHiddenInGame` _gameobject true)
    (`self.SetActorEnableCollision` _gameobject false)
    (`GameplayStatics.SpawnEmitterAtLocation` "/Game/StarterContent/Particles/P_SoundGong.P_SoundGong" (`self.K2_GetActorLocation` (`self.GameObject`)) (struct) (6.0 6.0 6.0))))

(event `ClosePetal`
  (`PrimitiveComponent.SetCollisionEnabled` (`self.Petal1`) "NoCollision")
  (`PrimitiveComponent.SetCollisionEnabled` (`self.Petal2`) "NoCollision")
  (`PrimitiveComponent.SetCollisionEnabled` (`self.Petal3`) "NoCollision")
  (`PrimitiveComponent.SetCollisionEnabled` (`self.Bulb`) "QueryAndPhysics"))

(event `ParasiteRemoved`
  (bind _health (`self.Health`))
  (`/Engine/EditorBlueprintResources/StandardMacros.DecrementInt` _health
    (:`  `
      (if (== _health 0)
        (if (`self.Unmoving`)
          (`self.OpenPetal`)
          (`KismetSystemLibrary.Delay` (`self.StayUpTime`))
          (`self.ClosePetal`)
          (elif (not (`self.Moving`))
            (`|ExecutionSequence`
              (:`then_0`
                (goto _label :!via `Reset`))
              (:`then_1`
                (`/Engine/EditorBlueprintResources/StandardMacros.DoOnce` false :!label _label
                  (:`Completed`
                    (`GameplayStatics.PlaySoundAtLocation` "/Game/_Sounds/Royalty_Free_Audio/AudioCues/S_GiantFlower_Cue.S_GiantFlower_Cue" (`self.K2_GetActorLocation`) (struct) 1.0 1.0 0.0 null null null)
                    (set `self.Moving` true)
                    (bind (_direction _swivel) (`Timeline|Timeline_0` :!label _label_2)
                      (:`Update`
                        (`SceneComponent.K2_SetRelativeLocation` (`self.Centre`) (`KismetMathLibrary.VLerp` (`self.StartVector`) (`self.EndVector`) (/ _swivel (`self.Speed`))) false false))
                      (:`Finished`
                        (`|ExecutionSequence`
                          (:`then_0`
                            (if (== _swivel 100.0)
                              (`self.OpenPetal`)
                              (else
                                (`self.ClosePetal`))))
                          (:`then_1`
                            (if (`self.Moving`)
                              (`KismetSystemLibrary.Delay` (`self.StayUpTime`))
                              (set `self.Moving` false)
                              (goto _label_2 :!via `Reverse`)
                              (else
                                (goto _label_2 :!via `SetNewTime`)))))))))))))))))

(fn `UserConstructionScript`)