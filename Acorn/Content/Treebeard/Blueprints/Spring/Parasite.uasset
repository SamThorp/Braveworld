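; Parasite is a destructible pumpkin-like growth that takes damage from seed hits and clears its linked Ivy when destroyed.
; Non-lethal hits briefly enlarge the pumpkin and swap its material, while BeginPlay configures a tougher, larger variant when BigParasite is set.
; On death it hides its meshes, darkens static-mesh ivy in timed material steps, then drops the Ivy far below and notifies Lily if flagged as LilyParasite.
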(event `self.ReceiveHit`
  (params (MyComp :type "PrimitiveComponent Object Reference") (Other :type "Actor Object Reference") (OtherComp :type "PrimitiveComponent Object Reference") (bSelfMoved :type Boolean) (HitLocation :type "Vector Structure") (HitNormal :type "Vector Structure") (NormalImpulse :type "Vector Structure") (Hit :type "HitResult Structure (by ref)"))
  (bind _pumpkin (`self.Pumpkin`))
  (bind _pumpkin_2 (`self.Pumpkin`))
  (bind _pumpkin_3 (`self.Pumpkin`))
  (bind _ivy (`self.Ivy`))
  (bind _returnvalue (`SceneComponent.K2_GetComponentLocation` _pumpkin_2))
  (bind _relativescale3d (`SceneComponent.RelativeScale3D` _pumpkin_3))
  (cast `/Game/Treebeard/Blueprints/Player/Seeds/AnySeed` Other)
  (bind _result (`/Engine/EditorBlueprintResources/StandardMacros.DecrementInt` (`self.HP`))
    (:`  `
      (if (<= _result 0)
        (`GameplayStatics.PlaySoundAtLocation` (`self.Sound`) _returnvalue (struct) 1.0 1.0 0.0 null null null)
        (`GameplayStatics.SpawnEmitterAtLocation` "/Game/InfinityBladeEffects/ForTreebeard/P_WaterBoomFlower.P_WaterBoomFlower" _returnvalue (`SceneComponent.K2_GetComponentRotation` _pumpkin_2) (4.0 4.0 4.0))
        (`SceneComponent.SetHiddenInGame` (`self.Pumpkin`) true false)
        (`SceneComponent.SetHiddenInGame` (`self.Ph2`) true false)
        (`SceneComponent.SetHiddenInGame` (`self.Psh3`) true false)
        (`self.SetActorEnableCollision` false)
        (`GameplayStatics.PlaySoundAtLocation` "/Game/_Sounds/Royalty_Free_Audio/AudioCues/S_IvyDestroy.S_IvyDestroy" (`self.K2_GetActorLocation` (`self.Ivy`)) (struct) 1.0 1.0 0.0 null null null)
        (bind _asstatic_mesh_actor (cast `StaticMeshActor` (`self.Ivy`))
          (:`then`
            (bind _staticmeshcomponent (`StaticMeshActor.StaticMeshComponent` _asstatic_mesh_actor))
            (`PrimitiveComponent.SetMaterial` _staticmeshcomponent 0 "/Game/_StylizedContent/Stylized_Landscape/materials/plants_materials/MI_vines_InstDarkA.MI_vines_InstDarkA")
            (`KismetSystemLibrary.Delay` 0.45)
            (`PrimitiveComponent.SetMaterial` _staticmeshcomponent 0 "/Game/_StylizedContent/Stylized_Landscape/materials/plants_materials/MI_vines_InstDarkB.MI_vines_InstDarkB")
            (`KismetSystemLibrary.Delay` 0.45)
            (`PrimitiveComponent.SetMaterial` _staticmeshcomponent 0 "/Game/_StylizedContent/Stylized_Landscape/materials/plants_materials/MI_vines_InstDarkC.MI_vines_InstDarkC")
            (`KismetSystemLibrary.Delay` 0.45))
          (:`CastFailed`
            (`KismetSystemLibrary.Delay` 0.9)
            (`GameplayStatics.SpawnEmitterAtLocation` "/Game/StarterContent/Particles/P_SoundGong.P_SoundGong" (`self.K2_GetActorLocation`) (struct) (2.0 2.0 2.0))))
        (`self.SetActorHiddenInGame` true)
        (`self.K2_SetActorLocation` _ivy (- (`self.K2_GetActorLocation` _ivy) (0.0 0.0 5000.0)) false false)
        (if (`self.LilyParasite`)
          (`/Game/Treebeard/Blueprints/Spring/GiantFlowerDeluxe.ParasiteRemoved` (`self.Lily`)))
        (else
          (`GameplayStatics.PlaySoundAtLocation` "/Game/_Sounds/Royalty_Free_Audio/AudioCues/S_ParasiteHit.S_ParasiteHit" (`self.K2_GetActorLocation`) (struct) 1.0 1.0 0.0 null null null)
          (`GameplayStatics.SpawnEmitterAtLocation` "/Game/InfinityBladeEffects/ForTreebeard/P_WaterBoomFlower.P_WaterBoomFlower" (`SceneComponent.K2_GetComponentLocation` _pumpkin) (`SceneComponent.K2_GetComponentRotation` _pumpkin) (1.5 1.5 1.5))
          (`SceneComponent.SetRelativeScale3D` _pumpkin_3 (+ _relativescale3d (0.2 0.2 0.2)))
          (`PrimitiveComponent.SetMaterial` _pumpkin_3 0 "/Game/_StylizedContent/AdvancedVillagePack/Materials/M_Inst_Pack_13.M_Inst_Pack_13")
          (`KismetSystemLibrary.Delay` 0.2)
          (`SceneComponent.SetRelativeScale3D` _pumpkin_3 (- _relativescale3d (0.2 0.2 0.2)))
          (`PrimitiveComponent.SetMaterial` _pumpkin_3 0 (`self.Material`)))))))

(event `self.ReceiveBeginPlay`
  (if (`self.BigParasite`)
    (`SceneComponent.SetRelativeScale3D` (`self.Pumpkin`) (1.5 1.5 1.5))
    (set `self.HP` 3)
    (`PrimitiveComponent.SetMaterial` (`self.Pumpkin`) 0 "/Game/_StylizedContent/AdvancedVillagePack/Materials/M_Inst_Pack_12.M_Inst_Pack_12")
    (`PrimitiveComponent.SetMaterial` (`self.Psh3`) 0 "/Game/_StylizedContent/AdvancedVillagePack/Materials/M_Inst_Pack_12.M_Inst_Pack_12")
    (`PrimitiveComponent.SetMaterial` (`self.Ph2`) 0 "/Game/_StylizedContent/AdvancedVillagePack/Materials/M_Inst_Pack_12.M_Inst_Pack_12")
    (set `self.Material` "/Game/_StylizedContent/AdvancedVillagePack/Materials/M_Inst_Pack_12.M_Inst_Pack_12")
    (set `self.Sound` "/Game/_Sounds/Royalty_Free_Audio/AudioCues/S_ParasiteDestroy_Cue_Large.S_ParasiteDestroy_Cue_Large")))

(fn `UserConstructionScript`)