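; BobbingTarget is a wrapper Blueprint around a Target child actor, passing its own settings into that target when play begins.
; BeginPlay casts the child actor to Target and copies charge, appear/disappear, permanence and game object settings before calling SetStuffUp.
; It then sets particle and scale and calls MaterialRing.
; The graphs hold no bobbing logic, and the construction script only calls its parent.
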(event `self.ReceiveBeginPlay`
  (`parent.ReceiveBeginPlay`)
  (bind _astarget (cast `/Game/Treebeard/Blueprints/Generic/Target` (`ChildActorComponent.ChildActor` (`self.ChildActor`))))
  (set `/Game/Treebeard/Blueprints/Generic/Target.Charged` (`self.Charged`) _astarget)
  (set `/Game/Treebeard/Blueprints/Generic/Target.DissapearOrAppear` (`self.DissapearOrAppear`) _astarget)
  (set `/Game/Treebeard/Blueprints/Generic/Target.Permanent` (`self.Permanent`) _astarget)
  (set `/Game/Treebeard/Blueprints/Generic/Target.GameObject` (`self.GameObject`) _astarget)
  (`/Game/Treebeard/Blueprints/Generic/Target.SetStuffUp` _astarget)
  (set `/Game/Treebeard/Blueprints/Generic/Target.Particle` (`self.Particle`) _astarget)
  (set `/Game/Treebeard/Blueprints/Generic/Target.Scale` (`self.Scale`) _astarget)
  (`/Game/Treebeard/Blueprints/Generic/Target.MaterialRing` _astarget))

(fn `UserConstructionScript`
  (`parent.UserConstructionScript`))