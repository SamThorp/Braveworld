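; Chargestone crystal that becomes temporarily charged when a SeedLightning actor hits its box, ignoring further hits until it resets.
; On a hit it swaps both crystal halves to the charged material and spawns a ChargingVolume timed to match the spark sequence.
; A self-calling delayed event emits lightning bursts at random points inside SparksHere, counting down sparks.
; After the last spark and a short pause, it restores the uncharged material and spark count.
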(event `self.ReceiveBeginPlay`
  (set `self.OriginalSparkCount` (`self.SparkCount`)))

(event `Flames`
  (bind _sparkshere (`self.SparksHere`))
  (bind _sparkcount (`self.SparkCount`))
  (bind _returnvalue (`GameplayStatics.SpawnEmitterAtLocation` "/Game/InfinityBladeEffects/ForTreebeard/P_RBurst_Lightning_Charge_01.P_RBurst_Lightning_Charge_01" (`KismetMathLibrary.RandomPointInBoundingBox` (`SceneComponent.K2_GetComponentLocation` _sparkshere) (`BoxComponent.GetScaledBoxExtent` _sparkshere)) :!label _label))
  (`/Engine/EditorBlueprintResources/StandardMacros.DecrementInt` _sparkcount
    (:`  `
      (`KismetSystemLibrary.Delay` (`self.SparkRate`))
      (if (<= _sparkcount 0)
        (`KismetSystemLibrary.Delay` 3.0)
        (set `self.Shocking` false)
        (`PrimitiveComponent.SetMaterial` (`self.CrystalTop`) 0 "/Game/StarterContent/Materials/M_CrystalUncharged.M_CrystalUncharged")
        (`PrimitiveComponent.SetMaterial` (`self.CrystalBottom`) 0 "/Game/StarterContent/Materials/M_CrystalUncharged.M_CrystalUncharged")
        (set `self.SparkCount` (`self.OriginalSparkCount`))
        (else
          (`self.Flames`))))))

(event `self.Box.OnComponentHit`
  (params (HitComponent :type "PrimitiveComponent Object Reference") (OtherActor :type "Actor Object Reference") (OtherComp :type "PrimitiveComponent Object Reference") (NormalImpulse :type "Vector Structure") (Hit :type "HitResult Structure (by ref)"))
  (cast `/Game/Treebeard/Blueprints/Player/Seeds/SeedLightning` OtherActor)
  (if (not (`self.Shocking`))
    (set `self.Shocking` true)
    (bind _returnvalue (`|SpawnActorFromClass` "/Game/Treebeard/Blueprints/Summer/ChargingVolume.ChargingVolume_C" (`KismetMathLibrary.Conv_VectorToTransform` (`self.K2_GetActorLocation` (`self.Actor`))) "Undefined" "OverrideRootScale" null null))
    (set `/Game/Treebeard/Blueprints/Summer/ChargingVolume.ActivityLength` (+ (* (`self.SparkCount`) (`self.SparkRate`)) 3.0) _returnvalue)
    (`PrimitiveComponent.SetMaterial` (`self.CrystalTop`) 0 "/Game/StarterContent/Materials/M_CrystalCharged.M_CrystalCharged")
    (`PrimitiveComponent.SetMaterial` (`self.CrystalBottom`) 0 "/Game/StarterContent/Materials/M_CrystalCharged.M_CrystalCharged")
    (goto _label)))

(fn `UserConstructionScript`)