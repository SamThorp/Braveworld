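; BurnableSurface is an actor that catches fire once when a SeedFire actor hits its box component.
; It then loops through the Flames event, spawning a flame emitter at a random point inside the box at each delayed step until the flame count runs out.
; After a final delay, it destroys its referenced Actor, if valid, and then itself.
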(event `self.Box.OnComponentHit`
  (params (HitComponent :type "PrimitiveComponent Object Reference") (OtherActor :type "Actor Object Reference") (OtherComp :type "PrimitiveComponent Object Reference") (NormalImpulse :type "Vector Structure") (Hit :type "HitResult Structure (by ref)"))
  (bind _actor (`self.Actor`))
  (bind _box (`self.Box`))
  (bind _flamecount (`self.FlameCount`))
  (cast `/Game/Treebeard/Blueprints/Player/Seeds/SeedFire` OtherActor)
  (if (not (`self.OnFire`))
    (set `self.OnFire` true)
    (`GameplayStatics.SpawnEmitterAtLocation` (`self.Flame`) (`KismetMathLibrary.RandomPointInBoundingBox` (`SceneComponent.K2_GetComponentLocation` _box) (`BoxComponent.GetScaledBoxExtent` _box)) :!label _label)
    (`/Engine/EditorBlueprintResources/StandardMacros.DecrementInt` _flamecount
      (:`  `
        (`KismetSystemLibrary.Delay` (`self.FlameRate`))
        (if (<= _flamecount 0)
          (`KismetSystemLibrary.Delay` 5.0)
          (`/Engine/EditorBlueprintResources/StandardMacros.IsValid` _actor
            (:`Is Valid`
              (`self.K2_DestroyActor` _actor))
            (:`Is Not Valid`
              _))
          (`self.K2_DestroyActor`)
          (else
            (`self.Flames`)))))))

(event `Flames`
  (goto _label))

(fn `UserConstructionScript`)