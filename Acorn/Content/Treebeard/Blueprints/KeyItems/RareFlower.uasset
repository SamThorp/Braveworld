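; RareFlower is a collectible key item: a potted plant that the main character picks up by touching it.
; Tick spins the Pot by a fixed yaw step each frame, independent of delta time.
; Overlapping Sphere1 reuses the character's CheckpointLevelName to show a congratulations message, then plays a pickup sound.
; It then flags its Index in the character's RareFlowers array and removes itself through a short lifespan.
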(event `self.ReceiveTick`
  (params (DeltaSeconds :type "Float (single-precision)"))
  (`SceneComponent.K2_AddRelativeRotation` (`self.Pot`) (struct :`Yaw` 0.5) false false))

(event `self.Sphere1.OnComponentBeginOverlap`
  (params (OverlappedComponent :type "PrimitiveComponent Object Reference") (OtherActor :type "Actor Object Reference") (OtherComp :type "PrimitiveComponent Object Reference") (OtherBodyIndex :type Integer) (bFromSweep :type Boolean) (SweepResult :type "HitResult Structure (by ref)"))
  (bind _asmain_character (cast `/Game/Treebeard/Blueprints/Player/MainCharacter` OtherActor))
  (`/Game/Treebeard/Blueprints/Player/MainCharacter.CheckpointLevelName` _asmain_character (`self.Congrats`) (`self.Tip`) "/Game/Font/Crazy_Cartoon_Font.Crazy_Cartoon_Font" 0.5)
  (`GameplayStatics.PlaySoundAtLocation` "/Game/_Sounds/Royalty_Free_Audio/AudioCues/S_PottedPlant_Cue.S_PottedPlant_Cue" (`self.K2_GetActorLocation`) (struct) 1.0 1.0 0.0 null null null)
  (`|ExecutionSequence`
    (:`then_0`
      (`KismetArrayLibrary.Array_Set` (`/Game/Treebeard/Blueprints/Player/MainCharacter.RareFlowers` _asmain_character) (`self.Index`) true))
    (:`then_1`
      (`self.SetLifeSpan` 0.1))))

(fn `UserConstructionScript`)