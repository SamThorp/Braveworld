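; DialgoueBP is an interactable that toggles an on-screen dialogue box when its InteractD event fires.
; If a dialogue widget is already open, it removes it and clears the reference.
; Otherwise it creates a WidgetDialgoue for player 0, adds it to the viewport and passes its MyText into the widget's DialogueText.
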(event `/Game/Better_Blueprints/Thorp/Dialogue/InterfaceDialogue.Interact D`
  (bind _dialoguewidget (`self.DialogueWidget`))
  (`/Engine/EditorBlueprintResources/StandardMacros.IsValid` _dialoguewidget
    (:`Is Valid`
      (`Widget.RemoveFromParent` _dialoguewidget)
      (set `self.DialogueWidget` null))
    (:`Is Not Valid`
      (bind _returnvalue (`|CreateWidget` "/Game/Better_Blueprints/Thorp/Dialogue/WidgetDialgoue.WidgetDialgoue_C" (`GameplayStatics.GetPlayerController` 0)))
      (bind _output_get (set `self.DialogueWidget` _returnvalue))
      (`UserWidget.AddToViewport` _output_get 0)
      (set `/Game/Better_Blueprints/Thorp/Dialogue/WidgetDialgoue.DialogueText` (`self.MyText`) (`self.DialogueWidget`)))))

(fn `UserConstructionScript`)