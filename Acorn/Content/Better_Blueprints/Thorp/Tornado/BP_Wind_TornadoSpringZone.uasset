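; Wandering tornado hazard that catches the player, carries them along a spline and flings them away.
; A looping timer picks a random point within the TornadoBounds actor's bounds, and Tick interpolates the root toward it with a sweep.
; On player overlap with TornadoCollision, a timeline moves the character along the spline by distance, keeping its rotation, then launches it in a random, scaled direction.
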(event `self.ReceiveBeginPlay`
  (`parent.ReceiveBeginPlay`)
  (bind _asmain_character (cast `/Game/Better_Blueprints/Treebeard/Blueprints/Player/MainCharacter` (`GameplayStatics.GetPlayerCharacter` 0)))
  (set `self.MainCharacterCast` _asmain_character)
  ;[1 1 1] Sets nado new location
  (`KismetSystemLibrary.K2_SetTimerDelegate` (delegate `MoveNado`) (`self.PositionChangeTime`) true))

(event `MoveNado`
  (bind (_origin _boxextent) (`KismetSystemLibrary.GetComponentBounds` (`Actor.RootComponent` (`self.Tornado Bounds`))))
  ;[1 1 1] Sets nado new location
  (set `self.NewLocation` (`KismetMathLibrary.RandomPointInBoundingBox` _origin _boxextent)))

(event `self.TornadoCollision.OnComponentBeginOverlap`
  (params (OverlappedComponent :type "PrimitiveComponent Object Reference") (OtherActor :type "Actor Object Reference") (OtherComp :type "PrimitiveComponent Object Reference") (OtherBodyIndex :type Integer) (bFromSweep :type Boolean) (SweepResult :type "HitResult Structure (by ref)"))
  (bind _spline (`self.Spline`))
  (bind _maincharactercast (`self.MainCharacterCast`))
  ;[1 1 1] Player Overlap
  (if (== OtherActor (`self.MainCharacterCast`))
    ;[1 1 1] Add player to Nado Spline
    (bind (_direction _progress) (`Timeline|Timeline_0` :!via `PlayFromStart`)
      (:`Update`
        (set `self.Nadoprogress` _progress)
        (`self.K2_SetActorLocationAndRotation` _maincharactercast (`SplineComponent.GetLocationAtDistanceAlongSpline` _spline (`KismetMathLibrary.Lerp` 0.0 (`SplineComponent.GetSplineLength` _spline) (`self.Nadoprogress`)) "World") (`self.K2_GetActorRotation` _maincharactercast) true false))
      (:`Finished`
        (`Character.LaunchCharacter` (`self.MainCharacterCast`) (* (`KismetMathLibrary.RandomUnitVector`) (3000.0 3000.0 2000.0)) true true)
        (set `self.Nadoprogress` 0.0)))))

(event `self.ReceiveTick`
  (params (DeltaSeconds :type "Float (single-precision)"))
  (bind _defaultsceneroot (`self.DefaultSceneRoot`))
  ;[1 1 1] Nado moves to new location
  (`SceneComponent.K2_SetWorldLocation` _defaultsceneroot (`KismetMathLibrary.VInterpTo` (`SceneComponent.K2_GetComponentLocation` _defaultsceneroot) (`self.NewLocation`) DeltaSeconds (`self.MovmentSpeed`)) true false))

(fn `UserConstructionScript`
  (`parent.UserConstructionScript`))