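; SwingingConker is a hanging conker hazard that knocks the main character away and can be broken with seeds.
; Sphere overlap launches the character away from the Scene component with clamped velocity, while a short DoOnce cooldown throttles sound and particles.
; Seed hits decrement HP, briefly flashing the material and enlarging the conker.
; At zero HP it bursts, hiding its meshes and disabling collision rather than destroying the actor.
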(event `self.Sphere.OnComponentBeginOverlap`
  (params (OverlappedComponent :type "PrimitiveComponent Object Reference") (OtherActor :type "Actor Object Reference") (OtherComp :type "PrimitiveComponent Object Reference") (OtherBodyIndex :type Integer) (bFromSweep :type Boolean) (SweepResult :type "HitResult Structure (by ref)"))
  (bind _returnvalue (`SceneComponent.K2_GetComponentLocation` (`self.Scene`)))
  (bind _asmain_character (cast `/Game/Better_Blueprints/Treebeard/Blueprints/Player/MainCharacter` OtherActor))
  (`Character.LaunchCharacter` _asmain_character (`KismetMathLibrary.ClampVectorSize` (* (- _returnvalue (`SceneComponent.K2_GetComponentLocation` (`Character.CapsuleComponent` _asmain_character))) -3.0) 0.0 2500.0) false false)
  (`/Engine/EditorBlueprintResources/StandardMacros.DoOnce` false :!label _label
    (:`Completed`
      (`GameplayStatics.SpawnSoundAtLocation` null _returnvalue (struct) 1.0 1.0 0.0 null null)
      (`GameplayStatics.SpawnEmitterAtLocation` null (`SceneComponent.K2_GetComponentLocation` (`self.Conker`)))
      (`KismetSystemLibrary.Delay` 0.2)
      (goto _label :!via `Reset`))))

(event `self.ReceiveHit`
  (params (MyComp :type "PrimitiveComponent Object Reference") (Other :type "Actor Object Reference") (OtherComp :type "PrimitiveComponent Object Reference") (bSelfMoved :type Boolean) (HitLocation :type "Vector Structure") (HitNormal :type "Vector Structure") (NormalImpulse :type "Vector Structure") (Hit :type "HitResult Structure (by ref)"))
  (bind _conker (`self.Conker`))
  (bind _conker_2 (`self.Conker`))
  (bind _conker_3 (`self.Conker`))
  (bind _relativescale3d (`SceneComponent.RelativeScale3D` _conker_3))
  (cast `/Game/Better_Blueprints/Treebeard/Blueprints/Player/Seeds/AnySeed` Other)
  (bind _result (`/Engine/EditorBlueprintResources/StandardMacros.DecrementInt` (`self.HP`))
    (:`  `
      (if (<= _result 0)
        (`GameplayStatics.SpawnEmitterAtLocation` null (`SceneComponent.K2_GetComponentLocation` _conker_2) (`SceneComponent.K2_GetComponentRotation` _conker_2) (1.5 1.5 1.5))
        (`SceneComponent.SetHiddenInGame` (`self.Knot1`) true false)
        (`SceneComponent.SetHiddenInGame` (`self.Rope`) true false)
        (`SceneComponent.SetHiddenInGame` (`self.Conker`) true false)
        (`self.SetActorEnableCollision` false)
        (`ActorComponent.K2_DestroyComponent` (`self.S_Conker_cue`))
        (`GameplayStatics.PlaySoundAtLocation` null (`SceneComponent.K2_GetComponentLocation` (`self.Conker`)) (struct) 1.0 1.0 0.0 null null null)
        (else
          (`GameplayStatics.SpawnEmitterAtLocation` null (`SceneComponent.K2_GetComponentLocation` _conker) (`SceneComponent.K2_GetComponentRotation` _conker) (1.5 1.5 1.5))
          (`SceneComponent.SetRelativeScale3D` _conker_3 (+ _relativescale3d (0.2 0.2 0.2)))
          (`PrimitiveComponent.SetMaterial` _conker_3 0 null)
          (`KismetSystemLibrary.Delay` 0.1)
          (`SceneComponent.SetRelativeScale3D` _conker_3 (- _relativescale3d (0.2 0.2 0.2)))
          (`PrimitiveComponent.SetMaterial` _conker_3 0 null))))))

(fn `UserConstructionScript`)