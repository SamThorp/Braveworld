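; A pumpkin target that catches fire and burns away when hit by a SeedFire actor.
; On BeginPlay it passes its own settings to a child Target actor and runs that actor's setup.
; The first hit plays a sound and starts a timed loop spawning flame emitters at random points inside a box.
; When the flame count runs out, it waits briefly, then destroys the pumpkin and box components.
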(event `self.ReceiveBeginPlay`
  (`parent.ReceiveBeginPlay`)
  (bind _astarget (cast `/Game/Better_Blueprints/Treebeard/Blueprints/Generic/Target` (`ChildActorComponent.ChildActor` (`self.ChildActor`))))
  (set `/Game/Better_Blueprints/Treebeard/Blueprints/Generic/Target.Charged` (`self.Charged`) _astarget)
  (set `/Game/Better_Blueprints/Treebeard/Blueprints/Generic/Target.DissapearOrAppear` (`self.DissapearOrAppear`) _astarget)
  (set `/Game/Better_Blueprints/Treebeard/Blueprints/Generic/Target.Permanent` (`self.Permanent`) _astarget)
  (set `/Game/Better_Blueprints/Treebeard/Blueprints/Generic/Target.GameObject` (`self.GameObject`) _astarget)
  (`/Game/Better_Blueprints/Treebeard/Blueprints/Generic/Target.SetStuffUp` _astarget)
  (set `/Game/Better_Blueprints/Treebeard/Blueprints/Generic/Target.Particle` (`self.Particle`) _astarget))

(event `self.Pumpkin.OnComponentHit`
  (params (HitComponent :type "PrimitiveComponent Object Reference") (OtherActor :type "Actor Object Reference") (OtherComp :type "PrimitiveComponent Object Reference") (NormalImpulse :type "Vector Structure") (Hit :type "HitResult Structure (by ref)"))
  (bind _pumpkin (`self.Pumpkin`))
  (bind _box (`self.Box`))
  (bind _flamecount (`self.FlameCount`))
  (bind _returnvalue (`SceneComponent.K2_GetComponentLocation` _box))
  (cast `/Game/Better_Blueprints/Treebeard/Blueprints/Player/Seeds/SeedFire` OtherActor)
  (if (not (`self.OnFire`))
    (set `self.OnFire` true)
    (`GameplayStatics.PlaySoundAtLocation` null _returnvalue (struct) 1.0 1.0 0.0 null null null)
    (`GameplayStatics.SpawnEmitterAtLocation` (`self.Flame`) (`KismetMathLibrary.RandomPointInBoundingBox` _returnvalue (`BoxComponent.GetScaledBoxExtent` _box)) :!label _label)
    (`/Engine/EditorBlueprintResources/StandardMacros.DecrementInt` _flamecount
      (:`  `
        (`KismetSystemLibrary.Delay` (`self.FlameRate`))
        (if (<= _flamecount 0)
          (`KismetSystemLibrary.Delay` 3.0)
          (`/Engine/EditorBlueprintResources/StandardMacros.IsValid` _pumpkin
            (:`Is Valid`
              (`ActorComponent.K2_DestroyComponent` _pumpkin)
              (`ActorComponent.K2_DestroyComponent` (`self.Box`))))
          (else
            (`self.Flames`)))))))

(event `Flames`
  (goto _label))

(fn `UserConstructionScript`
  (`parent.UserConstructionScript`))