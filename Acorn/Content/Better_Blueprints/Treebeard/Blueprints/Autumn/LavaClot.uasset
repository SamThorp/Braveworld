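; LavaClot is a lava hazard that kills the MainCharacter on overlapping its Cylinder and can be temporarily made solid with SeedWater.
; An unused SeedWater hitting the Box swaps both meshes' materials, enables the static mesh's collision and plays effects.
; A retriggerable delay, extended by repeat hits, then swaps materials again, disables that collision and plays effects.
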(event `OnHit`
  (params (OtherActor :type "Actor Object Reference"))
  (bind _returnvalue (`self.K2_GetActorLocation`))
  (bind _staticmeshcomponent (`self.StaticMeshComponent`))
  (bind _staticmeshcomponent_2 (`self.StaticMeshComponent`))
  (bind _staticmeshcomponent_3 (`self.StaticMeshComponent`))
  (bind _returnvalue_2 (`SceneComponent.K2_GetComponentLocation` _staticmeshcomponent))
  (bind _asseed_water (cast `/Game/Better_Blueprints/Treebeard/Blueprints/Player/Seeds/SeedWater` OtherActor))
  (if (not (`/Game/Better_Blueprints/Treebeard/Blueprints/Player/Seeds/SeedWater.Used` _asseed_water))
    (`PrimitiveComponent.SetMaterial` _staticmeshcomponent_3 0 null)
    (`PrimitiveComponent.SetMaterial` (`self.Cylinder`) 0 null)
    (`GameplayStatics.SpawnEmitterAtLocation` null _returnvalue_2 (`SceneComponent.K2_GetComponentRotation` _staticmeshcomponent) (1.5 1.5 1.5))
    (`GameplayStatics.PlaySoundAtLocation` null _returnvalue_2 (struct) 1.0 1.0 0.0 null null null)
    (`PrimitiveComponent.SetCollisionEnabled` _staticmeshcomponent_3 "QueryAndPhysics")
    (`KismetSystemLibrary.RetriggerableDelay` (`self.Duration`))
    (`PrimitiveComponent.SetMaterial` _staticmeshcomponent_2 0 null)
    (`PrimitiveComponent.SetMaterial` (`self.Cylinder`) 0 null)
    (`PrimitiveComponent.SetCollisionEnabled` _staticmeshcomponent_2 "NoCollision")
    (`GameplayStatics.PlaySoundAtLocation` null _returnvalue (struct) 1.0 1.0 0.0 null null null)
    (`GameplayStatics.SpawnEmitterAtLocation` null _returnvalue (struct) (* (`self.GetActorScale3D`) 10.0))))

(event `self.Box.OnComponentHit`
  (params (HitComponent :type "PrimitiveComponent Object Reference") (OtherActor :type "Actor Object Reference") (OtherComp :type "PrimitiveComponent Object Reference") (NormalImpulse :type "Vector Structure") (Hit :type "HitResult Structure (by ref)"))
  (`self.OnHit` OtherActor))

(event `self.Cylinder.OnComponentBeginOverlap`
  (params (OverlappedComponent :type "PrimitiveComponent Object Reference") (OtherActor :type "Actor Object Reference") (OtherComp :type "PrimitiveComponent Object Reference") (OtherBodyIndex :type Integer) (bFromSweep :type Boolean) (SweepResult :type "HitResult Structure (by ref)"))
  (bind _asmain_character (cast `/Game/Better_Blueprints/Treebeard/Blueprints/Player/MainCharacter` OtherActor))
  (`/Game/Better_Blueprints/Treebeard/Blueprints/Player/MainCharacter.Die` _asmain_character)
  (`GameplayStatics.PlaySoundAtLocation` null (`self.K2_GetActorLocation`) (struct) 1.0 1.0 0.0 null null null))

(fn `UserConstructionScript`)