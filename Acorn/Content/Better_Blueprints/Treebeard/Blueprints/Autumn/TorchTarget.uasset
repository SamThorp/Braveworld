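; TorchTarget is a torch that seed projectiles light or extinguish, toggling the visibility and collision of a linked GameObject.
; Capsule hits from SeedFire or SeedWater flip the Lit state, updating the fire visual, audio volume and a particle burst at the GameObject.
; DoThing shows or hides the GameObject with a sound, and AppearOnLit chooses whether lighting reveals it (hidden at start) or removes it.
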(event `self.ReceiveBeginPlay`
  (bind _gameobject (`self.GameObject`))
  (if (`self.AppearOnLit`)
    (`self.SetActorHiddenInGame` _gameobject true)
    (`self.SetActorEnableCollision` _gameobject false)))

(event `DoThing`
  (params (Branch :type Boolean))
  (bind _gameobject (`self.GameObject`))
  (bind _returnvalue (`self.K2_GetActorLocation` (`self.GameObject`)))
  (if Branch
    (`self.SetActorHiddenInGame` _gameobject true)
    (`self.SetActorEnableCollision` _gameobject false)
    (`GameplayStatics.PlaySoundAtLocation` null _returnvalue (struct) 1.0 1.0 0.0 null null null)
    (else
      (`self.SetActorHiddenInGame` _gameobject false)
      (`self.SetActorEnableCollision` _gameobject true)
      (`GameplayStatics.PlaySoundAtLocation` null _returnvalue (struct) 1.0 1.0 0.0 null null null))))

(event `self.Capsule.OnComponentHit`
  (params (HitComponent :type "PrimitiveComponent Object Reference") (OtherActor :type "Actor Object Reference") (OtherComp :type "PrimitiveComponent Object Reference") (NormalImpulse :type "Vector Structure") (Hit :type "HitResult Structure (by ref)"))
  (cast `/Game/Better_Blueprints/Treebeard/Blueprints/Player/Seeds/SeedFire` OtherActor
    (:`then`
      (if (not (`self.Lit`))
        (set `self.Lit` true)
        (`GameplayStatics.SpawnEmitterAtLocation` (`self.Particle`) (`self.K2_GetActorLocation` (`self.GameObject`)) (struct) (`self.Scale`))
        (`SceneComponent.SetVisibility` (`self.Fire1`) true false)
        (`self.DoThing` (== (`self.AppearOnLit`) false))
        (`AudioComponent.SetVolumeMultiplier` (`self.Audio`) 1.0)))
    (:`CastFailed`
      (cast `/Game/Better_Blueprints/Treebeard/Blueprints/Player/Seeds/SeedWater` OtherActor)
      (if (`self.Lit`)
        (set `self.Lit` false)
        (`GameplayStatics.SpawnEmitterAtLocation` (`self.Particle`) (`self.K2_GetActorLocation` (`self.GameObject`)) (struct) (`self.Scale`))
        (`SceneComponent.SetVisibility` (`self.Fire1`) false false)
        (`self.DoThing` (== (`self.AppearOnLit`) true))
        (`AudioComponent.SetVolumeMultiplier` (`self.Audio`) 0.0)))))

(fn `UserConstructionScript`)