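; Cannon actor that a SeedFire hit on its capsule lights, firing a single shot at an assigned GameObject.
; On BeginPlay it aims its Arrow at that target and, if AncientCannon is set, hides the AncientObjects and disables their collision.
; Once lit, it spawns a CannonBall and effects after a delay.
; A timed delay, not impact detection, then hides the target and reveals any AncientObjects.
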(event `self.ReceiveBeginPlay`
  (bind _ancientobjects (`self.AncientObjects`))
  (bind _arrow (`self.Arrow`))
  (bind _gameobject (`self.GameObject`))
  (`self.SetActorHiddenInGame` _gameobject false)
  (`self.SetActorEnableCollision` _gameobject true)
  (`SceneComponent.K2_SetWorldRotation` _arrow (`KismetMathLibrary.FindLookAtRotation` (`SceneComponent.K2_GetComponentLocation` _arrow) (`self.K2_GetActorLocation` _gameobject)) false false)
  (if (`self.AncientCannon`)
    (for _index (range (`KismetArrayLibrary.Array_Length` _ancientobjects))
      (bind _output (`|GetArrayItem` _ancientobjects _index))
      (`self.SetActorHiddenInGame` _output true)
      (`self.SetActorEnableCollision` _output false))))

(event `self.Capsule.OnComponentHit`
  (params (HitComponent :type "PrimitiveComponent Object Reference") (OtherActor :type "Actor Object Reference") (OtherComp :type "PrimitiveComponent Object Reference") (NormalImpulse :type "Vector Structure") (Hit :type "HitResult Structure (by ref)"))
  (cast `/Game/Better_Blueprints/Treebeard/Blueprints/Player/Seeds/SeedFire` OtherActor)
  (if (not (`self.Lit`))
    (set `self.Lit` true)
    (`SceneComponent.SetVisibility` (`self.Fire1`) true false)
    (`self.DoThing` false)
    (`GameplayStatics.PlaySoundAtLocation` null (`self.K2_GetActorLocation`) (struct) 1.0 1.0 0.0 null null null)))

(event `DoThing`
  (params (Branch :type Boolean))
  (bind _gameobject (`self.GameObject`))
  (bind _ancientobjects (`self.AncientObjects`))
  (bind _arrow (`self.Arrow`))
  (bind _returnvalue (`SceneComponent.K2_GetComponentLocation` _arrow))
  (`/Engine/EditorBlueprintResources/StandardMacros.DoOnce` false
    (:`Completed`
      (`KismetSystemLibrary.Delay` 1.0)
      (`|SpawnActorFromClass` "/Game/Better_Blueprints/Treebeard/Blueprints/Autumn/CannonBall.CannonBall_C" (`KismetMathLibrary.MakeTransform` _returnvalue (`SceneComponent.K2_GetComponentRotation` _arrow)) "Undefined" "OverrideRootScale" null null)
      (`GameplayStatics.SpawnEmitterAtLocation` null _returnvalue (struct) (2.0 2.0 2.0))
      (`KismetSystemLibrary.Delay` 0.2)
      (`GameplayStatics.SpawnEmitterAtLocation` (`self.Particle`) (`self.K2_GetActorLocation` (`self.GameObject`)) (struct) (`self.Scale`))
      (`self.SetActorHiddenInGame` _gameobject true)
      (`self.SetActorEnableCollision` _gameobject false)
      (`GameplayStatics.PlaySoundAtLocation` null (`self.K2_GetActorLocation`) (struct) 1.0 1.0 0.0 null null null)
      (if (`self.AncientCannon`)
        (for _index (range (`KismetArrayLibrary.Array_Length` _ancientobjects))
          (bind _output (`|GetArrayItem` _ancientobjects _index))
          (`self.SetActorHiddenInGame` _output false)
          (`self.SetActorEnableCollision` _output true))))))

(fn `UserConstructionScript`)