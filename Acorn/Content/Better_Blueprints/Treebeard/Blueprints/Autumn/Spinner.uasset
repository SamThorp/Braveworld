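; Physics spinner that moves a linked Platform actor between its starting position and an EndLocation offset from the spinner.
; A self-calling 0.01-second loop polls the Cube's Z angular velocity to play or reverse a timeline by spin direction, stopping it when spin is slow.
; The timeline lerps the platform's position, scaled by Speed.
; Mesh hits play a sound at the spinner and a rate-limited one at the platform.
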(event `self.ReceiveBeginPlay`
  (bind _endlocation_location (`KismetMathLibrary.BreakTransform` (`self.EndLocation`)))
  ;[1 1 1] Intial Setup of Locations
  (set `self.StartVector` (`self.K2_GetActorLocation` (`self.Platform`)))
  (set `self.EndVector` (+ (`self.K2_GetActorLocation`) _endlocation_location))
  (`self.GradualMove`))

(event `GradualMove`
  (bind (_returnvalue_x _returnvalue_y _returnvalue_z) (`KismetMathLibrary.BreakVector` (`PrimitiveComponent.GetPhysicsAngularVelocity` (`self.Cube`) "None")))
  (bind _returnvalue (> _returnvalue_z 50.0))
  ;[1 1 1] Spinning and Lifting
  (if _returnvalue
    (set `self.Reversal` false)
    (`|ExecutionSequence` :!label _label
      (:`then_0`
        (if (`self.Reversal`)
          (bind (_direction _swivel) (`Timeline|MoveTimeline` :!label _label_2)
            (:`Update`
              (`self.K2_SetActorRelativeLocation` (`self.Platform`) (`KismetMathLibrary.VLerp` (`self.StartVector`) (`self.EndVector`) (/ _swivel (`self.Speed`))) false false)))
          (else
            (goto _label_2 :!via `Reverse`))))
      (:`then_1`
        (`KismetSystemLibrary.Delay` 0.01 :!label _label_3)
        (`self.GradualMove`)))
    (elif (or _returnvalue (< _returnvalue_z -50.0))
      (set `self.Reversal` true)
      (goto _label)
      (else
        (`|ExecutionSequence`
          (:`then_0`
            (goto _label_2 :!via `Stop`))
          (:`then_1`
            (goto _label_3)))))))

(event `self.StaticMesh.OnComponentHit`
  (params (HitComponent :type "PrimitiveComponent Object Reference") (OtherActor :type "Actor Object Reference") (OtherComp :type "PrimitiveComponent Object Reference") (NormalImpulse :type "Vector Structure") (Hit :type "HitResult Structure (by ref)"))
  (`GameplayStatics.PlaySoundAtLocation` null (`self.K2_GetActorLocation`) (struct) 1.0 1.0 0.0 null null null :!label _label_4)
  (`/Engine/EditorBlueprintResources/StandardMacros.DoOnce` false :!label _label_5
    (:`Completed`
      (`GameplayStatics.PlaySoundAtLocation` null (`self.K2_GetActorLocation` (`self.Platform`)) (struct) 1.0 1.0 0.0 null null null)
      (`KismetSystemLibrary.Delay` 1.0)
      (goto _label_5 :!via `Reset`))))

(event `self.Cube.OnComponentHit`
  (params (HitComponent :type "PrimitiveComponent Object Reference") (OtherActor :type "Actor Object Reference") (OtherComp :type "PrimitiveComponent Object Reference") (NormalImpulse :type "Vector Structure") (Hit :type "HitResult Structure (by ref)"))
  (goto _label_4))

(fn `UserConstructionScript`)