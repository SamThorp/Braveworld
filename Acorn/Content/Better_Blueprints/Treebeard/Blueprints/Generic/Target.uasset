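; Target actor that shows or hides a linked GameObject, with sound and particles, when struck by a seed or pressed by the player or a PushBlock.
; Triggers work only while Charged, which overlapping a ChargingVolume grants temporarily.
; All triggers feed DoThing, gated by a DoOnce until Reset; DissapearOrAppear sets the direction.
; Setup applies charge-dependent meshes and materials, plus an Ice variant that jumps upward on hiding its object.
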(event `self.ReceiveBeginPlay`
  (bind _whitering (`self.WhiteRing`))
  (bind _bottombit (`self.BottomBit`))
  (bind _gameobject (`self.GameObject`))
  (`|ExecutionSequence` :!label _label
    (:`then_0`
      (if (not (`self.DissapearOrAppear`))
        (`self.SetActorHiddenInGame` _gameobject true)
        (`self.SetActorEnableCollision` _gameobject false)))
    (:`then_1`
      (if (not (`self.Charged`))
        (`PrimitiveComponent.SetMaterial` (`self.WhiteRing`) 0 null)
        (`PrimitiveComponent.SetMaterial` _bottombit 0 null)
        (`PrimitiveComponent.SetCollisionEnabled` _whitering "NoCollision")
        (`PrimitiveComponent.SetCollisionEnabled` (`self.RedDot`) "NoCollision")
        (`self.MakeHex` (`self.BottomBit`))
        (`self.MakeHex` (`self.RedRing`))
        (`self.MakeHex` (`self.RedDot`))
        (`self.MakeHex` _whitering)))
    (:`then_2`
      (if (`self.Ice`)
        (`PrimitiveComponent.SetMaterial` _bottombit 0 null)
        (`PrimitiveComponent.SetMaterial` (`self.RedRing`) 0 null)
        (`PrimitiveComponent.SetMaterial` (`self.RedDot`) 0 null)
        (set `self.OriginalLocation` (`self.K2_GetActorLocation`))))))

(event `MakeHex`
  (params (Target :type "StaticMeshComponent Object Reference"))
  (`StaticMeshComponent.SetStaticMesh` Target null))

(event `SetStuffUp`
  (goto _label))

(event `ReturnBackHome`
  (`self.K2_SetActorLocation` (`self.OriginalLocation`)))

(event `MaterialRing`
  (`PrimitiveComponent.SetMaterial` (`self.RedRing`) 0 (`self.MaterialForRings`))
  (`PrimitiveComponent.SetMaterial` (`self.RedDot`) 0 (`self.MaterialForRings`)))

(event `DoThing`
  (params (Branch :type Boolean))
  (bind _gameobject (`self.GameObject`))
  (bind _dissapearorappear (`self.DissapearOrAppear`))
  (bind _redring (`self.RedRing`))
  (bind _returnvalue (`self.K2_GetActorLocation` (`self.GameObject`)))
  (if (`self.Charged`)
    (`/Engine/EditorBlueprintResources/StandardMacros.DoOnce` false :!label _label_2
      (:`Completed`
        (`GameplayStatics.PlaySoundAtLocation` null (`self.K2_GetActorLocation`) (struct) 1.0 1.0 0.0 null null null)
        (`GameplayStatics.SpawnEmitterAtLocation` (`self.Particle`) (`self.K2_GetActorLocation` (`self.GameObject`)) (struct) (`self.Scale`))
        (if true
          (`SceneComponent.SetRelativeScale3D` _redring (0.8 0.8 2.0))
          (if _dissapearorappear
            (`self.SetActorHiddenInGame` _gameobject true :!label _label_3)
            (`self.SetActorEnableCollision` _gameobject false)
            (`GameplayStatics.PlaySoundAtLocation` null _returnvalue (struct) 1.0 1.0 0.0 null null null)
            (if (`self.Ice`)
              (`self.K2_AddActorLocalOffset` (0.0 0.0 500.0)))
            (else
              (`self.SetActorHiddenInGame` _gameobject false :!label _label_4)
              (`self.SetActorEnableCollision` _gameobject true)
              (`GameplayStatics.PlaySoundAtLocation` null _returnvalue (struct) 1.0 1.0 0.0 null null null)))
          (else
            (`SceneComponent.SetRelativeScale3D` _redring (0.8 0.8 5.0))
            (if _dissapearorappear
              (goto _label_4)
              (else
                (goto _label_3)))))))))

(event `Reset`
  (goto _label_2 :!via `Reset`))

(event `self.RedDot.OnComponentHit`
  (params (HitComponent :type "PrimitiveComponent Object Reference") (OtherActor :type "Actor Object Reference") (OtherComp :type "PrimitiveComponent Object Reference") (NormalImpulse :type "Vector Structure") (Hit :type "HitResult Structure (by ref)"))
  (cast `/Game/Better_Blueprints/Treebeard/Blueprints/Player/Seeds/AnySeed` OtherActor)
  (`self.DoThing` true :!label _label_5))

(event `self.RedRing.OnComponentHit`
  (params (HitComponent :type "PrimitiveComponent Object Reference") (OtherActor :type "Actor Object Reference") (OtherComp :type "PrimitiveComponent Object Reference") (NormalImpulse :type "Vector Structure") (Hit :type "HitResult Structure (by ref)"))
  (cast `/Game/Better_Blueprints/Treebeard/Blueprints/Player/Seeds/AnySeed` OtherActor)
  (goto _label_5))

(event `self.Sphere.OnComponentBeginOverlap`
  (params (OverlappedComponent :type "PrimitiveComponent Object Reference") (OtherActor :type "Actor Object Reference") (OtherComp :type "PrimitiveComponent Object Reference") (OtherBodyIndex :type Integer) (bFromSweep :type Boolean) (SweepResult :type "HitResult Structure (by ref)"))
  (bind _pointlight (`self.PointLight`))
  (bind _ascharging_volume (cast `/Game/Better_Blueprints/Treebeard/Blueprints/Summer/ChargingVolume` OtherActor))
  (`KismetSystemLibrary.Delay` 0.01)
  (set `self.Charged` true)
  (`SceneComponent.SetVisibility` _pointlight true false)
  (`PrimitiveComponent.SetMaterial` (`self.WhiteRing`) 0 null)
  (`KismetSystemLibrary.Delay` (`/Game/Better_Blueprints/Treebeard/Blueprints/Summer/ChargingVolume.ActivityLength` _ascharging_volume))
  (`KismetSystemLibrary.Delay` 0.2)
  (`PrimitiveComponent.SetMaterial` (`self.WhiteRing`) 0 null)
  (`SceneComponent.SetVisibility` _pointlight false false)
  (set `self.Charged` false))

(event `self.WhiteRing.OnComponentHit`
  (params (HitComponent :type "PrimitiveComponent Object Reference") (OtherActor :type "Actor Object Reference") (OtherComp :type "PrimitiveComponent Object Reference") (NormalImpulse :type "Vector Structure") (Hit :type "HitResult Structure (by ref)"))
  (cast `/Game/Better_Blueprints/Treebeard/Blueprints/Player/Seeds/AnySeed` OtherActor)
  (goto _label_5))

(event `PushDown`
  (params (Thing :type "Actor Object Reference"))
  (cast `/Game/Better_Blueprints/Treebeard/Blueprints/Player/MainCharacter` Thing
    (:`then`
      _)
    (:`CastFailed`
      (cast `/Game/Better_Blueprints/Treebeard/Blueprints/Generic/PushBlock` Thing)))
  (`self.DoThing` true)
  (`GameplayStatics.PlaySoundAtLocation` null (`self.K2_GetActorLocation`) (struct) 1.0 1.0 0.0 null null null :!label _label_6))

(event `PushUp`
  (params (Thing :type "Actor Object Reference"))
  (if (not (`self.Permanent`))
    (cast `/Game/Better_Blueprints/Treebeard/Blueprints/Player/MainCharacter` Thing
      (:`then`
        _)
      (:`CastFailed`
        (cast `/Game/Better_Blueprints/Treebeard/Blueprints/Generic/PushBlock` Thing)))
    (`self.DoThing` false)
    (goto _label_6)))

(fn `UserConstructionScript`)