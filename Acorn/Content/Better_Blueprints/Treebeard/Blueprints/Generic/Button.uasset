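; Pressure plate button that makes a linked GameObject disappear or appear, depending on DissapearOrAppear.
; Box overlaps keep a weight count, and MainCharacter or PushBlock overlaps lower or raise the platform.
; Activation requires charge from an overlapping ChargingVolume, which lights the button for that volume's ActivityLength.
; DoThing toggles visibility and collision with particle and sound; Permanent buttons destroy their trigger box once fired, others can revert.
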(event `self.ReceiveBeginPlay`
  (bind _gameobject (`self.GameObject`))
  (`|ExecutionSequence`
    (:`then_0`
      (if (not (`self.DissapearOrAppear`))
        (`self.SetActorHiddenInGame` _gameobject true)
        (`self.SetActorEnableCollision` _gameobject false))
      (set `self.OriginalLoc` (`SceneComponent.RelativeLocation` (`self.Platform`))))
    (:`then_1`
      (if (not (`self.Charged`))
        (`PrimitiveComponent.SetMaterial` (`self.BottomBit`) 0 null)))))

(event `DoThing`
  (params (ChargingVolume :type Boolean))
  (bind _gameobject (`self.GameObject`))
  (bind _platform (`self.Platform`))
  (bind _originalloc (`self.OriginalLoc`))
  (bind _dissapearorappear (`self.DissapearOrAppear`))
  (bind _returnvalue (`self.K2_GetActorLocation` (`self.GameObject`)))
  (if ChargingVolume
    _
    (elif (> (`self.WeightCount`) 0)
      (`SceneComponent.K2_SetRelativeLocation` _platform (- _originalloc (0.0 0.0 300.0)) false false)
      (if _dissapearorappear
        (if (`self.Charged`) :!label _label
          (`self.SetActorHiddenInGame` _gameobject true :!label _label_2)
          (`self.SetActorEnableCollision` _gameobject false)
          (if (`self.Permanent`) :!label _label_3
            (`/Engine/EditorBlueprintResources/StandardMacros.DoOnce` false
              (:`Completed`
                (`ActorComponent.K2_DestroyComponent` (`self.Box`)))))
          (if ChargingVolume
            _
            (elif (`self.Charged`)
              (`GameplayStatics.SpawnEmitterAtLocation` (`self.Particle`) (`self.K2_GetActorLocation` (`self.GameObject`)) (struct) (`self.Scale`))
              (if (`self.DissapearOrAppear`)
                (`GameplayStatics.PlaySoundAtLocation` null _returnvalue (struct) 1.0 1.0 0.0 null null null)
                (else
                  (`GameplayStatics.PlaySoundAtLocation` null _returnvalue (struct) 1.0 1.0 0.0 null null null)))))
          (elif (and (!= (`self.Permanent`) true) (!= (`self.DissapearOrAppear`) true))
            (goto _label_2)))
        (else
          (if (`self.Charged`) :!label _label_4
            (`self.SetActorHiddenInGame` _gameobject false :!label _label_5)
            (`self.SetActorEnableCollision` _gameobject true)
            (goto _label_3)
            (elif (and (!= (`self.Permanent`) true) (`self.DissapearOrAppear`))
              (goto _label_5)))))
      (else
        (`SceneComponent.K2_SetRelativeLocation` _platform _originalloc false false)
        (if _dissapearorappear
          (goto _label_4)
          (else
            (goto _label)))))))

(event `self.Box.OnComponentBeginOverlap`
  (params (OverlappedComponent :type "PrimitiveComponent Object Reference") (OtherActor :type "Actor Object Reference") (OtherComp :type "PrimitiveComponent Object Reference") (OtherBodyIndex :type Integer) (bFromSweep :type Boolean) (SweepResult :type "HitResult Structure (by ref)"))
  (`/Engine/EditorBlueprintResources/StandardMacros.IncrementInt` (`self.WeightCount`)
    (:`  `
      (`self.PushDown` OtherActor))))

(event `PushDown`
  (params (Thing :type "Actor Object Reference"))
  (bind _pointlight (`self.PointLight`))
  (bind _weightcount (`self.WeightCount`))
  (`|ExecutionSequence`
    (:`then_0`
      (bind _ascharging_volume (cast `/Game/Better_Blueprints/Treebeard/Blueprints/Summer/ChargingVolume` Thing)
        (:`then`
          (`KismetSystemLibrary.Delay` 0.01)
          (set `self.Charged` true)
          (`PrimitiveComponent.SetMaterial` (`self.BottomBit`) 0 null)
          (`/Engine/EditorBlueprintResources/StandardMacros.DecrementInt` _weightcount
            (:`  `
              (`SceneComponent.SetVisibility` _pointlight true false)
              (if (>= _weightcount 0)
                (if (> (`self.WeightCount`) 0)
                  (`self.DoThing` false)
                  (else
                    (`self.DoThing` true))))
              (`KismetSystemLibrary.Delay` (`/Game/Better_Blueprints/Treebeard/Blueprints/Summer/ChargingVolume.ActivityLength` _ascharging_volume))
              (`KismetSystemLibrary.Delay` 0.2)
              (`PrimitiveComponent.SetMaterial` (`self.BottomBit`) 0 null)
              (`SceneComponent.SetVisibility` _pointlight false false)
              (set `self.Charged` false))))
        (:`CastFailed`
          (cast `/Game/Better_Blueprints/Treebeard/Blueprints/Player/MainCharacter` Thing
            (:`then`
              _)
            (:`CastFailed`
              (cast `/Game/Better_Blueprints/Treebeard/Blueprints/Generic/PushBlock` Thing)))
          (`self.DoThing` false))))
    (:`then_1`
      (`GameplayStatics.PlaySoundAtLocation` null (`self.K2_GetActorLocation`) (struct) 1.0 1.0 0.0 null null null))))

(event `self.Box.OnComponentEndOverlap`
  (params (OverlappedComponent :type "PrimitiveComponent Object Reference") (OtherActor :type "Actor Object Reference") (OtherComp :type "PrimitiveComponent Object Reference") (OtherBodyIndex :type Integer))
  (cast `/Game/Better_Blueprints/Treebeard/Blueprints/Summer/ChargingVolume` OtherActor
    (:`then`
      _)
    (:`CastFailed`
      (`/Engine/EditorBlueprintResources/StandardMacros.DecrementInt` (`self.WeightCount`)
        (:`  `
          _))))
  (`self.PushUp` OtherActor))

(event `PushUp`
  (params (Thing :type "Actor Object Reference"))
  (`GameplayStatics.PlaySoundAtLocation` null (`self.K2_GetActorLocation`) (struct) 1.0 1.0 0.0 null null null)
  (if (`self.Permanent`)
    (if (not (`self.Charged`))
      (`SceneComponent.K2_SetRelativeLocation` (`self.Platform`) (`self.OriginalLoc`) false false))
    (else
      (cast `/Game/Better_Blueprints/Treebeard/Blueprints/Player/MainCharacter` Thing
        (:`then`
          (`self.DoThing` false :!label _label_6))
        (:`CastFailed`
          (cast `/Game/Better_Blueprints/Treebeard/Blueprints/Generic/PushBlock` Thing
            (:`then`
              (goto _label_6))
            (:`CastFailed`
              (cast `/Game/Better_Blueprints/Treebeard/Blueprints/Summer/ChargingVolume` Thing)
              (if (> (`self.WeightCount`) 0)
                (goto _label_6)
                (else
                  (`self.DoThing` true))))))))))

(fn `UserConstructionScript`)