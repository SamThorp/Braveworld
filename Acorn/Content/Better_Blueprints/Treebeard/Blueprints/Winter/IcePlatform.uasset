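; IcePlatform is a short-lived winter ice platform actor that breaks apart in two timed stages after spawning.
; On BeginPlay it plays a sound and randomizes Cylinder1's yaw and height offset for visual variation.
; After a delay it spawns particles and sound and destroys Cylinder2, then shortly afterwards plays a larger emitter with another sound and destroys itself.
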(event `self.ReceiveBeginPlay`
  (bind _returnvalue (`self.K2_GetActorLocation`))
  (bind _returnvalue_2 (`self.K2_GetActorLocation`))
  (`GameplayStatics.SpawnSoundAtLocation` null (`self.K2_GetActorLocation`) (struct) 1.0 1.0 0.0 null null)
  (`SceneComponent.K2_AddRelativeRotation` (`self.Cylinder1`) (`KismetMathLibrary.MakeRotator` 0.0 0.0 (`KismetMathLibrary.RandomFloatInRange` 0.0 280.0)) false false)
  (`SceneComponent.K2_AddRelativeLocation` (`self.Cylinder1`) (`KismetMathLibrary.MakeVector` 0.0 0.0 (`KismetMathLibrary.RandomFloatInRange` -2.0 5.0)) false false)
  (`KismetSystemLibrary.Delay` 8.0)
  (`GameplayStatics.SpawnEmitterAtLocation` null _returnvalue_2 (struct) (1.0 1.0 1.4))
  (`GameplayStatics.SpawnSoundAtLocation` null _returnvalue_2 (struct) 1.0 1.0 0.0 null null)
  (`ActorComponent.K2_DestroyComponent` (`self.Cylinder2`))
  (`KismetSystemLibrary.Delay` 2.0)
  (`GameplayStatics.SpawnSoundAtLocation` null _returnvalue (struct) 1.0 1.0 0.0 null null)
  (`GameplayStatics.SpawnEmitterAtLocation` null _returnvalue (struct) (2.0 2.0 2.0))
  (`self.K2_DestroyActor`))

(fn `UserConstructionScript`)