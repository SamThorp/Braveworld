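; Winter snowman statue puzzle that breaks apart once its three torches are lit by SeedFire projectiles.
; Each torch consumes the SeedFire and, only once, shows its flame, raises its audio and calls BreakLayer to destroy an ice mesh and decrement SnowmanHealth.
; At zero health, it fractures the destructible mesh with damage, plays effects and teleports the MoveThis actor far downward, then removes the debris after a delay.
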(event `self.ReceiveBeginPlay`
  (bind _snowmanmesh (`self.SnowmanMesh`))
  (`SceneComponent.SetVisibility` (`self.SnowmanDestructable`) true false)
  (`self.SetDestructibleMesh` (`self.SnowmanDestructable`) (`.DestructableMesh` (`self.DestructableMesh`)))
  (`StaticMeshComponent.SetStaticMesh` (`self.SnowmanIce1`) _snowmanmesh)
  (`StaticMeshComponent.SetStaticMesh` (`self.SnowmanIce2`) _snowmanmesh)
  (`StaticMeshComponent.SetStaticMesh` (`self.SnowmanIce3`) _snowmanmesh)
  (`PrimitiveComponent.SetMaterial` (`self.SnowmanIce2`) 0 null))

(event `BreakLayer`
  (params (Layer :type "StaticMeshComponent Object Reference") (Flame :type "ParticleSystemComponent Object Reference"))
  (bind _snowmanhealth (`self.SnowmanHealth`))
  (bind _movethis (`self.MoveThis`))
  (bind _snowmandestructable (`self.SnowmanDestructable`))
  (bind _returnvalue (`SceneComponent.K2_GetComponentLocation` _snowmandestructable))
  (`GameplayStatics.SpawnEmitterAtLocation` null (`SceneComponent.K2_GetComponentLocation` Layer) (struct) (1.5 1.5 1.5))
  (`ActorComponent.K2_DestroyComponent` Layer)
  (`/Engine/EditorBlueprintResources/StandardMacros.DecrementInt` _snowmanhealth
    (:`  `
      (`SceneComponent.SetVisibility` Flame true false)
      (if (== _snowmanhealth 0)
        (`KismetSystemLibrary.Delay` 1.0)
        (`SceneComponent.SetVisibility` (`self.SnowmanDestructable`) true false)
        (`GameplayStatics.ApplyDamage` _snowmandestructable null 0.0 null null null 20.0 _returnvalue _returnvalue 6.0)
        (`GameplayStatics.PlaySoundAtLocation` null _returnvalue (struct) 1.0 1.0 0.0 null null null)
        (`ActorComponent.K2_DestroyComponent` (`self.ParticleSystem`))
        (`ActorComponent.K2_DestroyComponent` (`self.Groundwork`))
        (`GameplayStatics.SpawnEmitterAtLocation` null (`self.K2_GetActorLocation` _movethis) (struct) (3.0 3.0 3.0))
        (`self.K2_AddActorLocalOffset` _movethis (0.0 0.0 -9000.0) false true)
        (`KismetSystemLibrary.Delay` 5.0)
        (`ActorComponent.K2_DestroyComponent` _snowmandestructable)))))

(event `self.Torch1.OnComponentHit`
  (params (HitComponent :type "PrimitiveComponent Object Reference") (OtherActor :type "Actor Object Reference") (OtherComp :type "PrimitiveComponent Object Reference") (NormalImpulse :type "Vector Structure") (Hit :type "HitResult Structure (by ref)"))
  (bind _asseed_fire (cast `/Game/Better_Blueprints/Treebeard/Blueprints/Player/Seeds/SeedFire` OtherActor))
  (`self.K2_DestroyActor` _asseed_fire)
  (`/Engine/EditorBlueprintResources/StandardMacros.DoOnce` false
    (:`Completed`
      (`self.BreakLayer` (`self.SnowmanIce1`) (`self.Fire1`))
      (`AudioComponent.SetVolumeMultiplier` (`self.Audio1`) 1.0))))

(event `self.Torch2.OnComponentHit`
  (params (HitComponent :type "PrimitiveComponent Object Reference") (OtherActor :type "Actor Object Reference") (OtherComp :type "PrimitiveComponent Object Reference") (NormalImpulse :type "Vector Structure") (Hit :type "HitResult Structure (by ref)"))
  (bind _asseed_fire (cast `/Game/Better_Blueprints/Treebeard/Blueprints/Player/Seeds/SeedFire` OtherActor))
  (`self.K2_DestroyActor` _asseed_fire)
  (`/Engine/EditorBlueprintResources/StandardMacros.DoOnce` false
    (:`Completed`
      (`self.BreakLayer` (`self.SnowmanIce2`) (`self.Fire2`))
      (`AudioComponent.SetVolumeMultiplier` (`self.Audio2`) 1.0))))

(event `self.Torch3.OnComponentHit`
  (params (HitComponent :type "PrimitiveComponent Object Reference") (OtherActor :type "Actor Object Reference") (OtherComp :type "PrimitiveComponent Object Reference") (NormalImpulse :type "Vector Structure") (Hit :type "HitResult Structure (by ref)"))
  (bind _asseed_fire (cast `/Game/Better_Blueprints/Treebeard/Blueprints/Player/Seeds/SeedFire` OtherActor))
  (`self.K2_DestroyActor` _asseed_fire)
  (`/Engine/EditorBlueprintResources/StandardMacros.DoOnce` false
    (:`Completed`
      (`self.BreakLayer` (`self.SnowmanIce3`) (`self.Fire3`))
      (`AudioComponent.SetVolumeMultiplier` (`self.Audio3`) 1.0))))

(fn `UserConstructionScript`)