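; Treebeard's face is the game's finale actor, celebrating once the player character has restored all four seasons.
; It polls the season flags every five seconds to swap its particle template.
; Capsule overlap with all seasons done shows a congratulations message, freezes movement, blends to a camera, plays a sound and recursively spawns bush "leaves" inside a box, then opens the main menu.
; LeavesHaha instead starts the leaf shower at BeginPlay and skips the menu load.
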(event `self.ReceiveBeginPlay`
  (if (`self.LeavesHaha`)
    (`self.Leaves`)
    (else
      (bind _asmain_character (cast `/Game/Better_Blueprints/Treebeard/Blueprints/Player/MainCharacter` (`GameplayStatics.GetPlayerCharacter` 0)))
      (`KismetSystemLibrary.Delay` 5.0 :!label _label)
      (if (and (`/Game/Better_Blueprints/Treebeard/Blueprints/Player/MainCharacter.WinterDone` _asmain_character) (`/Game/Better_Blueprints/Treebeard/Blueprints/Player/MainCharacter.AutumnDone` _asmain_character) (`/Game/Better_Blueprints/Treebeard/Blueprints/Player/MainCharacter.SpringDone` _asmain_character) (`/Game/Better_Blueprints/Treebeard/Blueprints/Player/MainCharacter.SummerDone` _asmain_character))
        (`ParticleSystemComponent.SetTemplate` (`self.ParticleSystemComponent`) null)
        (else
          (goto _label))))))

(event `self.Capsule.OnComponentBeginOverlap`
  (params (OverlappedComponent :type "PrimitiveComponent Object Reference") (OtherActor :type "Actor Object Reference") (OtherComp :type "PrimitiveComponent Object Reference") (OtherBodyIndex :type Integer) (bFromSweep :type Boolean) (SweepResult :type "HitResult Structure (by ref)"))
  (bind _asmain_character (cast `/Game/Better_Blueprints/Treebeard/Blueprints/Player/MainCharacter` OtherActor))
  (if (and (`/Game/Better_Blueprints/Treebeard/Blueprints/Player/MainCharacter.WinterDone` _asmain_character) (`/Game/Better_Blueprints/Treebeard/Blueprints/Player/MainCharacter.AutumnDone` _asmain_character) (`/Game/Better_Blueprints/Treebeard/Blueprints/Player/MainCharacter.SpringDone` _asmain_character) (`/Game/Better_Blueprints/Treebeard/Blueprints/Player/MainCharacter.SummerDone` _asmain_character))
    (`ParticleSystemComponent.SetTemplate` (`self.ParticleSystemComponent`) null)
    (`/Game/Better_Blueprints/Treebeard/Blueprints/Player/MainCharacter.CheckpointLevelName` _asmain_character "The Great Tree" "Congratulations! The Seasons have been restored." null 0.2)
    (`CharacterMovementComponent.DisableMovement` (`Character.CharacterMovement` _asmain_character))
    (`PlayerController.SetViewTargetWithBlend` (`GameplayStatics.GetPlayerController` 0) (`self.Camera`) 5.0 "VTBlend_Linear" 0.0 false)
    (`KismetSystemLibrary.Delay` 2.0)
    (`GameplayStatics.PlaySoundAtLocation` null (`self.K2_GetActorLocation`) (struct) 1.0 1.0 0.0 null null null)
    (`self.Leaves`)))

(event `Leaves`
  (bind _box (`self.Box`))
  (bind _leafcount (`self.LeafCount`))
  (`|SpawnActorFromClass` "/Game/Better_Blueprints/Treebeard/Blueprints/Spring/TreebeardBush.TreebeardBush_C" (`KismetMathLibrary.MakeTransform` (`KismetMathLibrary.RandomPointInBoundingBox` (`SceneComponent.K2_GetComponentLocation` _box) (`BoxComponent.GetScaledBoxExtent` _box)) (`KismetMathLibrary.RandomRotator` true)) "Undefined" "OverrideRootScale" null null)
  (`/Engine/EditorBlueprintResources/StandardMacros.DecrementInt` _leafcount
    (:`  `
      (`KismetSystemLibrary.Delay` (`self.LeafRate`))
      (if (<= _leafcount 0)
        (`KismetSystemLibrary.Delay` 10.0)
        (if (not (`self.LeavesHaha`))
          (`GameplayStatics.OpenLevel` "MainMenu"))
        (else
          (`self.Leaves`))))))

(fn `UserConstructionScript`)