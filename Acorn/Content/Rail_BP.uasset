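; Rail_BP is a spline-based rail actor that builds its track from meshes in the construction script, with no active event logic.
; For each SplineStruct entry, it steps along the spline in Divisor-length intervals and, if MeshOnOff is set, adds spline mesh components using that entry's mesh.
; Segment tangents are the spline direction offset by TangentFloat.
; ToolTipOnOff toggles the visibility of the Tip component.
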(fn `UserConstructionScript`
  (bind _tip (`self.Tip`))
  (bind _divisor (`self.Divisor`))
  (bind _spline (`self.Spline`))
  (bind _distance_a (`self.Distance A`))
  (bind _distance_b (`self.Distance B`))
  (if (`self.ToolTip On/Off`)
    (`SceneComponent.SetVisibility` _tip true false)
    (else
      (`SceneComponent.SetVisibility` _tip false false)))
  (for _index (range (+ (`KismetArrayLibrary.Array_Length` (`self.SplineStruct`)) 1))
    (bind (_mesh _divisor_2) (break `/Game/SplineStruct` (`|GetArrayItem` (`self.SplineStruct`) _index)))
    (set `self.Mesh` _mesh)
    (set `self.Divisor` _divisor_2)
    (for _index_2 (range (+ (`.ReturnValue` (`KismetMathLibrary.FMod` (`SplineComponent.GetSplineLength` (`self.Spline`)) (`self.Divisor`))) 1))
      (bind _returnvalue (* _index_2 _divisor))
      (set `self.Distance A` _returnvalue)
      (set `self.Distance B` (+ _returnvalue _divisor))
      (if (`self.Mesh On/Off`)
        (bind _returnvalue_2 (`AddComponent|NODE_AddSplineMeshComponent-0`))
        (`StaticMeshComponent.SetStaticMesh` _returnvalue_2 (`self.Mesh`))
        (`SplineMeshComponent.SetStartAndEnd` _returnvalue_2 (`SplineComponent.GetLocationAtDistanceAlongSpline` _spline _distance_a "Local") (+ (`SplineComponent.GetDirectionAtDistanceAlongSpline` _spline _distance_a "Local") (`self.Tangent float`)) (`SplineComponent.GetLocationAtDistanceAlongSpline` _spline _distance_b "Local") (+ (`SplineComponent.GetDirectionAtDistanceAlongSpline` _spline _distance_b "Local") (`self.Tangent float`)) true)))))