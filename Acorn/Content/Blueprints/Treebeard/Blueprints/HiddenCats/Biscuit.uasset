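; Biscuit is an actor in the HiddenCats folder that endlessly cycles a decorative attack animation with an ice impact effect.
; BeginPlay starts SwitchAxe, which plays the attack animation once and spawns the ice impact emitter at a Scene component's location partway through.
; It then switches the skeletal mesh to a looping idle, waits, and calls itself again, forming a timed loop built from Delays without Tick.
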(event `SwitchAxe`
  (bind _skeletalmeshcomponent (`self.SkeletalMeshComponent`))
  (`SkeletalMeshComponent.PlayAnimation` _skeletalmeshcomponent "/Game/Blueprints/Treebeard/Blueprints/HiddenCats/Animations/BiscuitATKPlayer_Anim.BiscuitATKPlayer_Anim" false)
  (`KismetSystemLibrary.Delay` 0.5)
  (`GameplayStatics.SpawnEmitterAtLocation` "/Game/InfinityBladeEffects/ForTreebeard/P_Impact_Ice.P_Impact_Ice" (`SceneComponent.K2_GetComponentLocation` (`self.Scene`)))
  (`KismetSystemLibrary.Delay` 0.5)
  (`SkeletalMeshComponent.PlayAnimation` _skeletalmeshcomponent "/Game/Blueprints/Treebeard/Blueprints/HiddenCats/Animations/BiscuitIdlePlayer_Anim.BiscuitIdlePlayer_Anim" true)
  (`KismetSystemLibrary.Delay` 3.0)
  (`self.SwitchAxe`))

(event `self.ReceiveBeginPlay`
  (`self.SwitchAxe`))

(fn `UserConstructionScript`)