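; FreezableSurface is an actor with a box collider that reacts to seed impacts and acts as water that can be frozen.
; An unused SeedIce hit spawns an IcePlatform at the impact point and marks the seed used, while a SeedLightning hit spawns a lightning bolt effect.
; When an overlapping MainCharacter is dead after a brief delay, it plays a water death sound, throttled by a timed DoOnce reset.
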(event `OnHit`
  (params (OtherActor :type "Actor Object Reference"))
  (bind _asseed_ice (cast `/Game/Blueprints/Treebeard/Blueprints/Player/Seeds/SeedIce` OtherActor)
    (:`then`
      (if (not (`/Game/Blueprints/Treebeard/Blueprints/Player/Seeds/SeedIce.Used` _asseed_ice))
        (`|SpawnActorFromClass` "/Game/Blueprints/Treebeard/Blueprints/Winter/IcePlatform.IcePlatform_C" (`KismetMathLibrary.Conv_VectorToTransform` (`.ImpactPoint` (`GameplayStatics.BreakHitResult` (stale `self.Box.OnComponentHit` Hit)))) "Undefined" "OverrideRootScale" null null)
        (set `/Game/Blueprints/Treebeard/Blueprints/Player/Seeds/SeedIce.Used` true _asseed_ice)))
    (:`CastFailed`
      (cast `/Game/Blueprints/Treebeard/Blueprints/Player/Seeds/SeedLightning` OtherActor)
      (`GameplayStatics.SpawnEmitterAtLocation` "/Game/InfinityBladeEffects/ForTreebeard/P_LightningBolt.P_LightningBolt" (`.ImpactPoint` (`GameplayStatics.BreakHitResult` (stale `self.Box.OnComponentHit` Hit)))))))

(event `self.Box.OnComponentHit`
  (params (HitComponent :type "PrimitiveComponent Object Reference") (OtherActor :type "Actor Object Reference") (OtherComp :type "PrimitiveComponent Object Reference") (NormalImpulse :type "Vector Structure") (Hit :type "HitResult Structure (by ref)"))
  (`self.OnHit` OtherActor))

(event `self.Box.OnComponentBeginOverlap`
  (params (OverlappedComponent :type "PrimitiveComponent Object Reference") (OtherActor :type "Actor Object Reference") (OtherComp :type "PrimitiveComponent Object Reference") (OtherBodyIndex :type Integer) (bFromSweep :type Boolean) (SweepResult :type "HitResult Structure (by ref)"))
  (bind _asmain_character (cast `/Game/Blueprints/Treebeard/Blueprints/Player/MainCharacter` OtherActor))
  (`/Engine/EditorBlueprintResources/StandardMacros.IsValid` _asmain_character
    (:`Is Valid`
      (`KismetSystemLibrary.Delay` 0.1)
      (if (`/Game/Blueprints/Treebeard/Blueprints/Player/MainCharacter.Dead` _asmain_character)
        (`/Engine/EditorBlueprintResources/StandardMacros.DoOnce` false :!label _label
          (:`Completed`
            (`GameplayStatics.PlaySoundAtLocation` "/Game/_Sounds/Royalty_Free_Audio/AudioCues/S_DeathWater.S_DeathWater" (`self.K2_GetActorLocation` _asmain_character) (struct) 1.0 1.0 0.0 null null null)
            (`KismetSystemLibrary.Delay` 3.3)
            (goto _label :!via `Reset`)))))))

(fn `UserConstructionScript`)