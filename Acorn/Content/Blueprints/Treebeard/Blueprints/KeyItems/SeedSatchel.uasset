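; SeedSatchel is a key-item pickup that unlocks one elemental seed type for the MainCharacter.
; Overlapping Sphere1 calls the character's CheckpointLevelName with congrats and tip text, then WhichElement selects the Water, Thunder, Fire or Ice seed flag to set.
; It then refreshes HUDPc visibility for non-controller players, plays a pickup sound and expires via a short lifespan.
; Tick slowly rotates the Sphere component.
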(event `self.ReceiveTick`
  (params (DeltaSeconds :type "Float (single-precision)"))
  (`SceneComponent.K2_AddRelativeRotation` (`self.Sphere`) (struct :`Yaw` 0.5) false false))

(event `self.Sphere1.OnComponentBeginOverlap`
  (params (OverlappedComponent :type "PrimitiveComponent Object Reference") (OtherActor :type "Actor Object Reference") (OtherComp :type "PrimitiveComponent Object Reference") (OtherBodyIndex :type Integer) (bFromSweep :type Boolean) (SweepResult :type "HitResult Structure (by ref)"))
  (bind _asmain_character (cast `/Game/Blueprints/Treebeard/Blueprints/Player/MainCharacter` OtherActor))
  (`/Game/Blueprints/Treebeard/Blueprints/Player/MainCharacter.CheckpointLevelName` _asmain_character (`self.Congrats`) (`self.Tip`) "/Game/Font/Frostys_Winterland_Font.Frostys_Winterland_Font" 0.5)
  (`|ExecutionSequence`
    (:`then_0`
      (switch `int` (`self.WhichElement`)
        (:`Default`
          (set `/Game/Blueprints/Treebeard/Blueprints/Player/MainCharacter.GotIceSeeds` true _asmain_character :!label _label))
        (:`0`
          (set `/Game/Blueprints/Treebeard/Blueprints/Player/MainCharacter.GotWaterSeeds` true _asmain_character :!label _label_2))
        (:`1`
          (goto _label_2))
        (:`2`
          (set `/Game/Blueprints/Treebeard/Blueprints/Player/MainCharacter.GotThunderSeeds` true _asmain_character))
        (:`3`
          (set `/Game/Blueprints/Treebeard/Blueprints/Player/MainCharacter.GotFireSeeds` true _asmain_character))
        (:`4`
          (goto _label))))
    (:`then_1`
      (if (not (`/Game/Blueprints/Treebeard/Blueprints/Player/MainCharacter.UsingController` _asmain_character))
        (`/Game/Blueprints/Treebeard/Blueprints/Player/UI/HUDPC.CheckVisibility` (`/Game/Blueprints/Treebeard/Blueprints/Player/MainCharacter.HUDPc` _asmain_character))))
    (:`then_2`
      (`GameplayStatics.PlaySoundAtLocation` "/Game/_Sounds/Royalty_Free_Audio/AudioCues/S_SeedSatchel_Cue.S_SeedSatchel_Cue" (`self.K2_GetActorLocation`) (struct) 1.0 1.0 0.0 null null null)
      (`self.SetLifeSpan` 0.1))))

(fn `UserConstructionScript`)