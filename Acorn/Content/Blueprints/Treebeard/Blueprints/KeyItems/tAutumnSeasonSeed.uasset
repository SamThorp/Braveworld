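; Autumn season seed key item: a spinning pickup that triggers when the MainCharacter overlaps it.
; Overlap shows a congratulatory tip via CheckpointLevelName, plays the autumn cue and passes its SkyRotation to the character.
; A WhichSeason switch updates the character's season flags, setting only AutumnDone true and clearing the matching flag in other cases.
; It then expires both the RemoveThis actor and itself through short lifespans.
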(event `self.ReceiveTick`
  (params (DeltaSeconds :type "Float (single-precision)"))
  (`SceneComponent.K2_AddRelativeRotation` (`self.Sphere`) (struct :`Yaw` 0.8) false false))

(event `self.Sphere1.OnComponentBeginOverlap`
  (params (OverlappedComponent :type "PrimitiveComponent Object Reference") (OtherActor :type "Actor Object Reference") (OtherComp :type "PrimitiveComponent Object Reference") (OtherBodyIndex :type Integer) (bFromSweep :type Boolean) (SweepResult :type "HitResult Structure (by ref)"))
  (bind _asmain_character (cast `/Game/Blueprints/Treebeard/Blueprints/Player/MainCharacter` OtherActor))
  (`/Game/Blueprints/Treebeard/Blueprints/Player/MainCharacter.CheckpointLevelName` _asmain_character (`self.Congrats`) (`self.Tip`) "/Game/Font/Frostys_Winterland_Font.Frostys_Winterland_Font" 0.5)
  (`GameplayStatics.PlaySoundAtLocation` "/Game/_Sounds/Royalty_Free_Audio/AudioCues/S_SeasonalSeedCue_Autumn.S_SeasonalSeedCue_Autumn" (`self.K2_GetActorLocation`) (struct) 1.0 1.0 0.0 null null null)
  (set `/Game/Blueprints/Treebeard/Blueprints/Player/MainCharacter.SkyRotation` (`self.SkyRotation`) _asmain_character)
  (`|ExecutionSequence`
    (:`then_0`
      (switch `int` (`self.WhichSeason`)
        (:`Default`
          (set `/Game/Blueprints/Treebeard/Blueprints/Player/MainCharacter.WinterDone` false _asmain_character :!label _label))
        (:`0`
          (set `/Game/Blueprints/Treebeard/Blueprints/Player/MainCharacter.SpringDone` false _asmain_character :!label _label_2))
        (:`1`
          (goto _label_2))
        (:`2`
          (set `/Game/Blueprints/Treebeard/Blueprints/Player/MainCharacter.SummerDone` false _asmain_character))
        (:`3`
          (set `/Game/Blueprints/Treebeard/Blueprints/Player/MainCharacter.AutumnDone` true _asmain_character))
        (:`4`
          (goto _label))))
    (:`then_1`
      (`self.SetLifeSpan` (`self.RemoveThis`) 0.1)
      (`self.SetLifeSpan` 0.1))))

(fn `UserConstructionScript`)