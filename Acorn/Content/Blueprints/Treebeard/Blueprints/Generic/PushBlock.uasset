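; PushBlock is a block whose resistance to sliding changes as the MainCharacter enters or leaves its XBOX and YBOX trigger volumes.
; On overlap, the Cube's linear damping is set to Weight so the player can push it.
; When an overlap ends, damping becomes very high to halt the block, or low if Icy so it keeps sliding.
; The delayed damping check after an icy release has no effect.
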(event `self.ReceiveBeginPlay`)

(event `self.YBOX.OnComponentBeginOverlap`
  (params (OverlappedComponent :type "PrimitiveComponent Object Reference") (OtherActor :type "Actor Object Reference") (OtherComp :type "PrimitiveComponent Object Reference") (OtherBodyIndex :type Integer) (bFromSweep :type Boolean) (SweepResult :type "HitResult Structure (by ref)"))
  (cast `/Game/Blueprints/Treebeard/Blueprints/Player/MainCharacter` OtherActor)
  (`PrimitiveComponent.SetLinearDamping` (`self.Cube`) (`self.Weight`) :!label _label) ; Sets the linear dampening (how slidy) the object is
)

(event `self.XBOX.OnComponentBeginOverlap`
  (params (OverlappedComponent :type "PrimitiveComponent Object Reference") (OtherActor :type "Actor Object Reference") (OtherComp :type "PrimitiveComponent Object Reference") (OtherBodyIndex :type Integer) (bFromSweep :type Boolean) (SweepResult :type "HitResult Structure (by ref)"))
  (cast `/Game/Blueprints/Treebeard/Blueprints/Player/MainCharacter` OtherActor)
  (goto _label))

(event `self.XBOX.OnComponentEndOverlap`
  (params (OverlappedComponent :type "PrimitiveComponent Object Reference") (OtherActor :type "Actor Object Reference") (OtherComp :type "PrimitiveComponent Object Reference") (OtherBodyIndex :type Integer))
  (bind _cube (`self.Cube`))
  (cast `/Game/Blueprints/Treebeard/Blueprints/Player/MainCharacter` OtherActor)
  (if (`self.Icy`) :!label _label_2
    (`PrimitiveComponent.SetLinearDamping` _cube 0.6) ; Sets the linear dampening (how slidy) the object is
    (`KismetSystemLibrary.RetriggerableDelay` 1.0)
    (if (== (`self.Weight`) (`PrimitiveComponent.GetLinearDamping` _cube))
      _)
    (else
      (`PrimitiveComponent.SetLinearDamping` _cube 5000.0) ; Sets the linear dampening (how slidy) the object is
    )))

(event `self.YBOX.OnComponentEndOverlap`
  (params (OverlappedComponent :type "PrimitiveComponent Object Reference") (OtherActor :type "Actor Object Reference") (OtherComp :type "PrimitiveComponent Object Reference") (OtherBodyIndex :type Integer))
  (cast `/Game/Blueprints/Treebeard/Blueprints/Player/MainCharacter` OtherActor)
  (goto _label_2))

(fn `UserConstructionScript`)