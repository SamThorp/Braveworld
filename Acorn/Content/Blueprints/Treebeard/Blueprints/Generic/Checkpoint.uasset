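; Checkpoint actor shown as a flower that saves the MainCharacter's respawn point when the player overlaps its capsule.
; If the player is falling, it rechecks every quarter second during overlap and activates only once they are grounded.
; Activation closes the previous checkpoint's flower, opens this one, swaps particles, plays a sound and stores the player's location and Respawn value on the character.
; It can optionally display the world and location name through the character.
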(event `self.ReceiveBeginPlay`
  (`SceneComponent.SetVisibility` (`self.ParticleSystem1`) false false))

(event `self.Capsule.OnComponentBeginOverlap`
  (params (OverlappedComponent :type "PrimitiveComponent Object Reference") (OtherActor :type "Actor Object Reference") (OtherComp :type "PrimitiveComponent Object Reference") (OtherBodyIndex :type Integer) (bFromSweep :type Boolean) (SweepResult :type "HitResult Structure (by ref)"))
  (bind _asmain_character (cast `/Game/Blueprints/Treebeard/Blueprints/Player/MainCharacter` OtherActor))
  (if (`NavMovementComponent.IsFalling` (`Character.CharacterMovement` _asmain_character)) :!label _label
    (`KismetSystemLibrary.Delay` 0.25)
    (if (`PrimitiveComponent.IsOverlappingActor` (`self.Capsule`) OtherActor)
      (goto _label))
    (else
      (bind _checkpoint (`/Game/Blueprints/Treebeard/Blueprints/Player/MainCharacter.Checkpoint` _asmain_character))
      (`/Engine/EditorBlueprintResources/StandardMacros.IsValid` _checkpoint
        (:`Is Valid`
          (if (!= _checkpoint self)
            (set `/Game/Blueprints/Treebeard/Blueprints/Generic/Checkpoint.CurrentCheck` false (`/Game/Blueprints/Treebeard/Blueprints/Player/MainCharacter.Checkpoint` _asmain_character))
            (`SkeletalMeshComponent.PlayAnimation` (`/Game/Blueprints/Treebeard/Blueprints/Generic/Checkpoint.SkeletalMesh` _checkpoint) "/Game/_ProjectTreebeard/ElenaModels/Lily/FlowerAnimClose_Anim.FlowerAnimClose_Anim" false)
            (`SceneComponent.SetVisibility` (`/Game/Blueprints/Treebeard/Blueprints/Generic/Checkpoint.ParticleSystem` _checkpoint) true false)
            (`SceneComponent.SetVisibility` (`/Game/Blueprints/Treebeard/Blueprints/Generic/Checkpoint.ParticleSystem1` _checkpoint) false false)
            (set `/Game/Blueprints/Treebeard/Blueprints/Player/MainCharacter.Checkpoint` self _asmain_character :!label _label_2)
            (set `/Game/Blueprints/Treebeard/Blueprints/Player/MainCharacter.SpawnHere` (`self.K2_GetActorLocation` _asmain_character) _asmain_character)
            (set `self.CurrentCheck` true)
            (`SceneComponent.SetVisibility` (`self.ParticleSystem`) false false)
            (`SkeletalMeshComponent.PlayAnimation` (`self.SkeletalMesh`) "/Game/_ProjectTreebeard/ElenaModels/Lily/FlowerAnimOpen_Anim.FlowerAnimOpen_Anim" false)
            (`SceneComponent.SetVisibility` (`self.ParticleSystem1`) true false)
            (set `/Game/Blueprints/Treebeard/Blueprints/Player/MainCharacter.Respawn` (`self.Respawn`) _asmain_character)
            (`GameplayStatics.PlaySoundAtLocation` "/Game/_Sounds/Royalty_Free_Audio/AudioCues/S_Checkpoint_Cue.S_Checkpoint_Cue" (`self.K2_GetActorLocation`) (struct) 1.0 1.0 0.0 null null null)
            (if (`self.SaysLevelName`)
              (`/Game/Blueprints/Treebeard/Blueprints/Player/MainCharacter.CheckpointLevelName` _asmain_character (`self.WorldName`) (`self.LocationName`) (`self.Level Font`) 1.01))))
        (:`Is Not Valid`
          (goto _label_2))))))

(fn `UserConstructionScript`)