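; LavaClot is a lava hazard that kills the MainCharacter on overlapping its Cylinder and can be temporarily frozen into stone.
; An unused SeedWater hitting the Box swaps the materials to stone, enables mesh collision, and plays freeze effects.
; A retriggerable Duration delay then restores lava, disables mesh collision, and plays break sound and explosion, so repeated hits extend the frozen state.
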(event `OnHit`
  (params (OtherActor :type "Actor Object Reference"))
  (bind _returnvalue (`self.K2_GetActorLocation`))
  (bind _staticmeshcomponent (`self.StaticMeshComponent`))
  (bind _staticmeshcomponent_2 (`self.StaticMeshComponent`))
  (bind _staticmeshcomponent_3 (`self.StaticMeshComponent`))
  (bind _returnvalue_2 (`SceneComponent.K2_GetComponentLocation` _staticmeshcomponent))
  (bind _asseed_water (cast `/Game/Blueprints/Treebeard/Blueprints/Player/Seeds/SeedWater` OtherActor))
  (if (not (`/Game/Blueprints/Treebeard/Blueprints/Player/Seeds/SeedWater.Used` _asseed_water))
    (`PrimitiveComponent.SetMaterial` _staticmeshcomponent_3 0 "/Game/_StylizedContent/lost_island/Materials/stones_materials/MI_stone_B_Inst2.MI_stone_B_Inst2")
    (`PrimitiveComponent.SetMaterial` (`self.Cylinder`) 0 "/Game/_StylizedContent/lost_island/Materials/stones_materials/MI_stone_B_Inst2.MI_stone_B_Inst2")
    (`GameplayStatics.SpawnEmitterAtLocation` "/Game/StarterContent/Particles/P_SoundGong.P_SoundGong" _returnvalue_2 (`SceneComponent.K2_GetComponentRotation` _staticmeshcomponent) (1.5 1.5 1.5))
    (`GameplayStatics.PlaySoundAtLocation` "/Game/_Sounds/Royalty_Free_Audio/AudioCues/S_LavaClotCue_Freeze.S_LavaClotCue_Freeze" _returnvalue_2 (struct) 1.0 1.0 0.0 null null null)
    (`PrimitiveComponent.SetCollisionEnabled` _staticmeshcomponent_3 "QueryAndPhysics")
    (`KismetSystemLibrary.RetriggerableDelay` (`self.Duration`))
    (`PrimitiveComponent.SetMaterial` _staticmeshcomponent_2 0 "/Game/_StylizedContent/scorched_land/materials/lava_materials/MI_lava_A_Inst1.MI_lava_A_Inst1")
    (`PrimitiveComponent.SetMaterial` (`self.Cylinder`) 0 "/Game/_StylizedContent/scorched_land/materials/lava_materials/MI_lava_A_Inst1.MI_lava_A_Inst1")
    (`PrimitiveComponent.SetCollisionEnabled` _staticmeshcomponent_2 "NoCollision")
    (`GameplayStatics.PlaySoundAtLocation` "/Game/_Sounds/Royalty_Free_Audio/AudioCues/S_LavaClotCue_Break.S_LavaClotCue_Break" _returnvalue (struct) 1.0 1.0 0.0 null null null)
    (`GameplayStatics.SpawnEmitterAtLocation` "/Game/StarterContent/Particles/P_Explosion.P_Explosion" _returnvalue (struct) (* (`self.GetActorScale3D`) 10.0))))

(event `self.Box.OnComponentHit`
  (params (HitComponent :type "PrimitiveComponent Object Reference") (OtherActor :type "Actor Object Reference") (OtherComp :type "PrimitiveComponent Object Reference") (NormalImpulse :type "Vector Structure") (Hit :type "HitResult Structure (by ref)"))
  (`self.OnHit` OtherActor))

(event `self.Cylinder.OnComponentBeginOverlap`
  (params (OverlappedComponent :type "PrimitiveComponent Object Reference") (OtherActor :type "Actor Object Reference") (OtherComp :type "PrimitiveComponent Object Reference") (OtherBodyIndex :type Integer) (bFromSweep :type Boolean) (SweepResult :type "HitResult Structure (by ref)"))
  (bind _asmain_character (cast `/Game/Blueprints/Treebeard/Blueprints/Player/MainCharacter` OtherActor))
  (`/Game/Blueprints/Treebeard/Blueprints/Player/MainCharacter.Die` _asmain_character)
  (`GameplayStatics.PlaySoundAtLocation` "/Game/_Sounds/Royalty_Free_Audio/AudioCues/S_DeathLava.S_DeathLava" (`self.K2_GetActorLocation`) (struct) 1.0 1.0 0.0 null null null))

(fn `UserConstructionScript`)