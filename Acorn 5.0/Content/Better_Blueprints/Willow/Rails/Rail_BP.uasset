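; Rail actor that builds spline meshes along an editable spline and reacts when the main character overlaps it.
; The construction script loops over each mesh and divisor entry, tiling spline mesh segments at that spacing, with an optional tooltip and mesh toggle.
; Spline overlap launches the character at a constant negative velocity, since the two identical arrow vectors cancel, and prints a debug "Hello".
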(event `self.Spline.OnComponentBeginOverlap`
  (params (OverlappedComponent :type "PrimitiveComponent Object Reference") (OtherActor :type "Actor Object Reference") (OtherComp :type "PrimitiveComponent Object Reference") (OtherBodyIndex :type Integer) (bFromSweep :type Boolean) (SweepResult :type "HitResult Structure (by ref)"))
  (bind _asmain_character (cast `/Game/Better_Blueprints/Treebeard/Blueprints/Player/MainCharacter` OtherActor))
  (bind _arrow2 (`/Game/Better_Blueprints/Treebeard/Blueprints/Player/MainCharacter.Arrow2` _asmain_character))
  (`Character.LaunchCharacter` _asmain_character (- (- (`SceneComponent.GetForwardVector` _arrow2) (`SceneComponent.GetForwardVector` _arrow2)) 50.0) true true)
  (`KismetSystemLibrary.PrintString` "Hello"))

(fn `UserConstructionScript`
  (bind _tip (`self.Tip`))
  (bind _divisor (`self.Divisor`))
  (bind _spline (`self.Spline`))
  (bind _distance_a (`self.Distance A`))
  (bind _distance_b (`self.Distance B`))
  (if (`self.ToolTip On/Off`)
    (`SceneComponent.SetVisibility` _tip true false)
    (else
      (`SceneComponent.SetVisibility` _tip false false)))
  (for _index (range (+ (`KismetArrayLibrary.Array_Length` (`self.SplineStruct`)) 1))
    (bind (_mesh _divisor_2) (break `/Game/Better_Blueprints/Willow/Rails/SplineStruct` (`|GetArrayItem` (`self.SplineStruct`) _index)))
    (set `self.Mesh` _mesh)
    (set `self.Divisor` _divisor_2)
    (for _index_2 (range (+ (`.ReturnValue` (`KismetMathLibrary.FMod` (`SplineComponent.GetSplineLength` (`self.Spline`)) (`self.Divisor`))) 1))
      (bind _returnvalue (* _index_2 _divisor))
      (set `self.Distance A` _returnvalue)
      (set `self.Distance B` (+ _returnvalue _divisor))
      (if (`self.Mesh On/Off`)
        (bind _returnvalue_2 (`AddComponent|NODE_AddSplineMeshComponent-0`))
        (`StaticMeshComponent.SetStaticMesh` _returnvalue_2 (`self.Mesh`))
        (`SplineMeshComponent.SetStartAndEnd` _returnvalue_2 (`SplineComponent.GetLocationAtDistanceAlongSpline` _spline _distance_a "Local") (+ (`SplineComponent.GetDirectionAtDistanceAlongSpline` _spline _distance_a "Local") (`self.Tangent float`)) (`SplineComponent.GetLocationAtDistanceAlongSpline` _spline _distance_b "Local") (+ (`SplineComponent.GetDirectionAtDistanceAlongSpline` _spline _distance_b "Local") (`self.Tangent float`)) true)))))