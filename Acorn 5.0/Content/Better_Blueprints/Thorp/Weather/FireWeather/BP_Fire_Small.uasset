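; BP_Fire_Small is a short-lived fire that can grow into a big fire, with particles driven by the player character's wind direction and speed.
; After a short delay it line-traces vertically at its Plane and spawns BP_Fire_Big on Grass or Wood physical surfaces.
; It skips spawning when the player's FireAmount cap is reached or a BP_BigFire is hit.
; It destroys itself within seconds, or on overlapping a Water-tagged actor.
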(event `self.ReceiveBeginPlay`
  (bind _p_fire_small_converted (`self.P_Fire_Small_Converted`))
  (bind _asmain_character (cast `/Game/Better_Blueprints/Treebeard/Blueprints/Player/MainCharacter` (`GameplayStatics.GetPlayerCharacter` 0)))
  (bind _output_get (set `self.As Main Character_0` _asmain_character))
  (`FXSystemComponent.SetVectorParameter` _p_fire_small_converted "Direction" (`/Game/Better_Blueprints/Treebeard/Blueprints/Player/MainCharacter.Wind_Rot_MC` _output_get))
  (`FXSystemComponent.SetFloatParameter` _p_fire_small_converted "FireAngleLimit" (* 0.05 (`/Game/Better_Blueprints/Treebeard/Blueprints/Player/MainCharacter.Wind_Speed_MC` _output_get)))
  (`KismetSystemLibrary.Delay` 1.0)
  (`self.Propagate`))

(event `Propagate`
  (bind _returnvalue (`SceneComponent.K2_GetComponentLocation` (`self.Plane`)))
  (bind (_returnvalue_x _returnvalue_y) (`KismetMathLibrary.BreakVector` (`SceneComponent.K2_GetComponentLocation` (`self.Plane`))))
  (if (not (`self.StopPropagate`))
    (`/Engine/EditorBlueprintResources/StandardMacros.IncrementInt` (`self.PropogatedCount`)
      (:`  `
        (`|ExecutionSequence`
          (:`then_0`
            (if (>= (`/Game/Better_Blueprints/Treebeard/Blueprints/Player/MainCharacter.Fire Amount` (`self.As Main Character_0`)) 10)
              (`self.K2_DestroyActor`)
              (else
                (bind (_outhit _returnvalue_2) (`KismetSystemLibrary.LineTraceSingle` (+ _returnvalue (0.0 0.0 100.0)) (+ _returnvalue (0.0 0.0 -100.0)) "TraceTypeQuery1"))
                (if _returnvalue_2
                  (bind (_bblockinghit _binitialoverlap _time _distance _location _impactpoint _normal _impactnormal _physmat _hitactor) (`GameplayStatics.BreakHitResult` _outhit))
                  (bind _asbp_big_fire (cast `/Game/Better_Blueprints/Thorp/Weather/FireWeather/BP_BigFire` _hitactor)
                    (:`then`
                      (if (== _asbp_big_fire _hitactor)
                        (`self.K2_DestroyActor`)
                        (else
                          (switch `EPhysicalSurface` (`PhysicalMaterial.SurfaceType` _physmat) :!label _label
                            (:`SurfaceType_Default`
                              _)
                            (:`SurfaceType1`
                              (`|SpawnActorFromClass` "/Game/Better_Blueprints/Thorp/Weather/FireWeather/BP_Fire_Big.BP_Fire_Big_C" (`KismetMathLibrary.MakeTransform` (`KismetMathLibrary.MakeVector` _returnvalue_x _returnvalue_y (.z _location)) (`KismetMathLibrary.MakeRotator` 0.0)) "Undefined" "OverrideRootScale" null null :!label _label_2))
                            (:`SurfaceType2`
                              _)
                            (:`SurfaceType3`
                              _)
                            (:`SurfaceType4`
                              (goto _label_2))
                            (:`SurfaceType5`
                              _)
                            (:`SurfaceType6`
                              _)
                            (:`SurfaceType7`
                              _))
                          (`KismetSystemLibrary.Delay` 5.0)
                          (`self.K2_DestroyActor`))))
                    (:`CastFailed`
                      (goto _label)))
                  (else
                    (`KismetSystemLibrary.Delay` 5.0)
                    (`self.K2_DestroyActor`))))))
          (:`then_1`
            (`KismetSystemLibrary.Delay` 5.0)
            (`self.K2_DestroyActor`)))))))

(event `self.ReceiveDestroyed`)

(event `self.ReceiveActorBeginOverlap`
  (params (OtherActor :type "Actor Object Reference"))
  (if (`self.ActorHasTag` OtherActor "Water")
    (`self.K2_DestroyActor`)))

(fn `UserConstructionScript`
  (`parent.UserConstructionScript`))