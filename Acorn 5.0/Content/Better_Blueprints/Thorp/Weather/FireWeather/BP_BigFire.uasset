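; BP_BigFire is a weather-system fire actor that destroys itself when overlapped by an actor tagged Water.
; BeginPlay and Propagate are empty, so its wind and spreading logic is disconnected and never runs.
; That dormant logic sets Niagara fire direction from player wind, traces to spawn BP_Fire on Grass or Wood, then swaps effects in stages before destroying itself.
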(event `self.ReceiveBeginPlay`)

(event `self.ReceiveActorBeginOverlap`
  (params (OtherActor :type "Actor Object Reference"))
  (if (`self.ActorHasTag` OtherActor "Water")
    (`self.K2_DestroyActor`)))

(event `Propagate`)

(fn `UserConstructionScript`)