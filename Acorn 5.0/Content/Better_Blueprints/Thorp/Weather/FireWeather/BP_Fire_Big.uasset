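; Big weather fire that spreads by spawning BP_Fire_Small on nearby grass or wood, then dies down.
; On begin it increments the player's FireAmount and sets effect direction and angle from the player's wind.
; Five timed, wind-biased random steps line-trace the ground, skipping existing fires, with stronger wind shortening the interval.
; It then decrements FireAmount, swaps through burn-down effects and destroys itself; touching Water-tagged actors destroys it immediately, without decrementing.
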(event `self.ReceiveBeginPlay`
  (bind _p_fire_small_converted (`self.P_Fire_Small_Converted`))
  (bind _as_main_character_0 (`self.As Main Character_0`))
  (bind _asmain_character (cast `/Game/Better_Blueprints/Treebeard/Blueprints/Player/MainCharacter` (`GameplayStatics.GetPlayerCharacter` 0))
    (:`then`
      (bind _output_get (set `self.As Main Character_0` _asmain_character))
      (set `/Game/Better_Blueprints/Treebeard/Blueprints/Player/MainCharacter.Fire Amount` (+ (`/Game/Better_Blueprints/Treebeard/Blueprints/Player/MainCharacter.Fire Amount` _as_main_character_0) 1) _as_main_character_0)
      (`FXSystemComponent.SetVectorParameter` _p_fire_small_converted "Direction" (`/Game/Better_Blueprints/Treebeard/Blueprints/Player/MainCharacter.Wind_Rot_MC` _output_get))
      (`FXSystemComponent.SetFloatParameter` _p_fire_small_converted "FireAngleLimit" (* 0.05 (`/Game/Better_Blueprints/Treebeard/Blueprints/Player/MainCharacter.Wind_Speed_MC` _output_get))))
    (:`CastFailed`
      _))
  (set `self.FireArray` (`|MakeArray` "/Game/M5VFXVOL2/Niagara/Fire_for_Dir/NFire_Dir_00.NFire_Dir_00" "/Game/M5VFXVOL2/Niagara/Fire_for_Dir/NFire_Dir_01.NFire_Dir_01" "/Game/M5VFXVOL2/Niagara/Fire_for_Dir/NFire_Dir_02.NFire_Dir_02" "/Game/M5VFXVOL2/Niagara/Fire_for_Dir/NFire_Dir_03.NFire_Dir_03" "/Game/M5VFXVOL2/Niagara/Fire_for_Dir/NFire_Dir_04.NFire_Dir_04" "/Game/M5VFXVOL2/Niagara/Fire_for_Dir/NFire_Dir_05.NFire_Dir_05" "/Game/M5VFXVOL2/Niagara/Fire_for_Dir/NFire_Dir_06.NFire_Dir_06" "/Game/M5VFXVOL2/Niagara/Fire_for_Dir/NFire_Dir_07.NFire_Dir_07" "/Game/M5VFXVOL2/Niagara/Fire_for_Dir/NFire_Dir_08.NFire_Dir_08" "/Game/M5VFXVOL2/Niagara/Fire_for_Dir/NFire_Dir_09.NFire_Dir_09" "/Game/M5VFXVOL2/Niagara/Fire_for_Dir/NFire_Dir_10.NFire_Dir_10" "/Game/M5VFXVOL2/Niagara/Fire_for_Dir/NFire_Dir_11.NFire_Dir_11" "/Game/M5VFXVOL2/Niagara/Fire_for_Dir/NFire_Dir_12.NFire_Dir_12" :!type "NiagaraSystem Object Reference"))
  (`KismetSystemLibrary.Delay` 1.0)
  (`self.Propagate`))

(event `self.ReceiveActorBeginOverlap`
  (params (OtherActor :type "Actor Object Reference"))
  (if (`self.ActorHasTag` OtherActor "Water")
    (`self.K2_DestroyActor`)))

(event `Propagate`
  (bind _as_main_character_0 (`self.As Main Character_0`))
  (bind (_propagatelocal_x _propagatelocal_y) (`KismetMathLibrary.BreakVector` (`self.PropagateLocal`)))
  (if (not (`self.StopPropagate`))
    (`/Engine/EditorBlueprintResources/StandardMacros.IncrementInt` (`self.PropogatedCount`)
      (:`  `
        (`|ExecutionSequence`
          (:`then_0`
            (bind _output_get (set `self.PropagateLocal` (+ (* (+ (select `int` (`KismetMathLibrary.RandomInteger` 4) :`0` (2.0 0.0 0.0) :`1` (2.0 2.0 0.0) :`2` (-2.0 0.0 0.0) :`3` (-2.0 -2.0 0.0) :`4` (2.0 0.0 0.0) :!type "Vector Structure") (`/Game/Better_Blueprints/Treebeard/Blueprints/Player/MainCharacter.Wind_Rot_MC` (`self.As Main Character_0`))) 50.0) (`self.K2_GetActorLocation`))))
            (bind (_outhit _returnvalue) (`KismetSystemLibrary.LineTraceSingle` (+ _output_get (0.0 0.0 100.0)) (+ _output_get (0.0 0.0 -100.0)) "TraceTypeQuery1"))
            (if _returnvalue
              (bind (_bblockinghit _binitialoverlap _time _distance _location _impactpoint _normal _impactnormal _physmat _hitactor) (`GameplayStatics.BreakHitResult` _outhit))
              (cast `/Game/Better_Blueprints/Thorp/Weather/FireWeather/BP_Fire` _hitactor
                (:`CastFailed`
                  (cast `/Game/Better_Blueprints/Thorp/Weather/FireWeather/BP_BigFire` _hitactor
                    (:`CastFailed`
                      (switch `EPhysicalSurface` (`PhysicalMaterial.SurfaceType` _physmat)
                        (:`SurfaceType1`
                          _)
                        (:`SurfaceType4`
                          _))
                      (`|SpawnActorFromClass` "/Game/Better_Blueprints/Thorp/Weather/FireWeather/BP_Fire_Small.BP_Fire_Small_C" (`KismetMathLibrary.MakeTransform` (`KismetMathLibrary.MakeVector` _propagatelocal_x _propagatelocal_y (.z _location)) (`KismetMathLibrary.MakeRotator` 0.0 0.0 (`KismetMathLibrary.RandomFloatInRange` 0.0 360.0))) "Undefined" "OverrideRootScale" null null)))))))
          (:`then_1`
            (`KismetSystemLibrary.Delay` (- 5.1 (/ (`/Game/Better_Blueprints/Treebeard/Blueprints/Player/MainCharacter.Wind_Speed_MC` (`self.As Main Character_0`)) 2.0)))
            (if (< (`self.PropogatedCount`) 5)
              (`self.Propagate`)
              (else
                (set `/Game/Better_Blueprints/Treebeard/Blueprints/Player/MainCharacter.Fire Amount` (- (`/Game/Better_Blueprints/Treebeard/Blueprints/Player/MainCharacter.Fire Amount` _as_main_character_0) 1) _as_main_character_0)
                (`NiagaraComponent.SetAsset` (`self.P_Fire_Small_Converted`) (`KismetArrayLibrary.Array_Random` (`self.FireArray`)) false)
                (set `self.StopPropagate` true)
                (`KismetSystemLibrary.Delay` 10.0)
                (`NiagaraComponent.SetAsset` (`self.P_Fire_Small_Converted`) "/Game/M5VFXVOL2/Niagara/Fire_for_Dir/NFire_Grd_Dir_02.NFire_Grd_Dir_02" false)
                (`KismetSystemLibrary.Delay` 10.0)
                (`NiagaraComponent.SetAsset` (`self.P_Fire_Small_Converted`) "/Game/M5VFXVOL2/Niagara/Fire_for_Dir/NFire_Grd_Dir_01.NFire_Grd_Dir_01" false)
                (`KismetSystemLibrary.Delay` 10.0)
                (`NiagaraComponent.SetAsset` (`self.P_Fire_Small_Converted`) "/Game/M5VFXVOL2/Niagara/Fire_for_Dir/NFire_Grd_Dir_00.NFire_Grd_Dir_00" false)
                (`KismetSystemLibrary.Delay` 10.0)
                (`self.K2_DestroyActor`)))))))))

(fn `UserConstructionScript`
  (`parent.UserConstructionScript`))